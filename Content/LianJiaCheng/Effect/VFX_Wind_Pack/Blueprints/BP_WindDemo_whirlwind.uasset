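; BP_WindDemo_whirlwind is a demo whirlwind effect actor that travels along a referenced spline.
; After a short startup delay, if activated, a timeline scaled by a duration and offset by a start time drives its position and rotation along the full spline length.
; Overlapping a BP_WindDemo_sphere deactivates and hides the whirlwind effect.
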(event `self.ReceiveBeginPlay`
  (`KismetSystemLibrary.Delay` 3.0)
  (if (`self.Activate`)
    (`self.MoveAlong`)))

(event `MoveAlong`
  (bind _returnvalue (`KismetMathLibrary.Lerp` 0.0 (`SplineComponent.GetSplineLength` (`/Game/LianJiaCheng/Effect/VFX_Wind_Pack/Blueprints/BP_WindDemo_Spline.Spline` (`self.SplineRef`))) (`self.Alpha`)))
  (`TimelineComponent.SetPlayRate` (`self.Timeline`) (/ 1.0 (`self.Duration`)))
  (`TimelineComponent.SetNewTime` (`self.Timeline`) (`self.TimelineStart`))
  (bind (_direction _alpha) (`Timeline|Timeline`)
    (:`Update`
      (set `self.Alpha` _alpha)
      (`self.K2_SetActorLocationAndRotation` (`SplineComponent.GetLocationAtDistanceAlongSpline` (`/Game/LianJiaCheng/Effect/VFX_Wind_Pack/Blueprints/BP_WindDemo_Spline.Spline` (`self.SplineRef`)) _returnvalue "World") (`SplineComponent.GetRotationAtDistanceAlongSpline` (`/Game/LianJiaCheng/Effect/VFX_Wind_Pack/Blueprints/BP_WindDemo_Spline.Spline` (`self.SplineRef`)) _returnvalue "World")))))

(event `self.ReceiveActorBeginOverlap`
  (params (OtherActor :type "Actor Object Reference"))
  (cast `/Game/LianJiaCheng/Effect/VFX_Wind_Pack/Blueprints/BP_WindDemo_sphere` OtherActor)
  (`ActorComponent.Deactivate` (`self.Whirlwind`))
  (`SceneComponent.SetVisibility` (`self.Whirlwind`) false false))

(fn `UserConstructionScript`)