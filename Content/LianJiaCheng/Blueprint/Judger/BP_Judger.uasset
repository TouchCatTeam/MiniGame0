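; BP_Judger is the central referee for slime fights, breeding and target selection.
; Slimes are queued for death, birth or hunt, and Tick resolves one entry or pair per queue.
; Death rolls both slimes against class-matchup rates; births use pair rates gated by birth delay.
; Hunts search a slime list refreshed every second, giving males the nearest enemy and females the nearest same-side female, skipping the last one hit.
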(event `self.ReceiveBeginPlay`
  (`self.GetAllSlimes`))

(event `/Game/LianJiaCheng/Blueprint/Judger/BPI_Judger.AddDeathQuene`
  (params (ObjAttacked :type "Actor Object Reference") (ObjAttacking :type "Actor Object Reference"))
  (bind _inputreadyquene1 (`self.InputReadyQuene1`))
  ;[1 1 1] Add Quene
  (`KismetArrayLibrary.Array_Add` _inputreadyquene1 ObjAttacked)
  (`KismetArrayLibrary.Array_Add` _inputreadyquene1 ObjAttacking))

(event `/Game/LianJiaCheng/Blueprint/Judger/BPI_Judger.AddBirthQuene`
  (params (Obj1 :type "Actor Object Reference") (Obj2 :type "Actor Object Reference"))
  (bind _inputreadyquene2 (`self.InputReadyQuene2`))
  ;[1 1 1] Add Quene
  (`KismetArrayLibrary.Array_Add` _inputreadyquene2 Obj1)
  (`KismetArrayLibrary.Array_Add` _inputreadyquene2 Obj2))

(event `/Game/LianJiaCheng/Blueprint/Judger/BPI_Judger.AddHuntQuene`
  (params (Hunter :type "Actor Object Reference"))
  ;[1 1 1] Add Quene
  (`KismetArrayLibrary.Array_Add` (`self.HuntQuene`) Hunter))

(event `self.ReceiveTick`
  (params (DeltaSeconds :type "Float (single-precision)"))
  ;[1 1 1] Handle Quene Every Tick
  (`|ExecutionSequence`
    (:`then_0`
      (if (not (== (`KismetArrayLibrary.Array_Length` (`self.InputReadyQuene1`)) 0))
        (`self.HandleFirstTwoInDeathQuene`)
        ;[1 1 1] Play Hit Sound
        (`GameplayStatics.PlaySound2D` "/Game/LianJiaCheng/Sound/SCue_Hit.SCue_Hit" 1.0 1.0 0.0 null null)))
    (:`then_1`
      (if (not (== (`KismetArrayLibrary.Array_Length` (`self.InputReadyQuene2`)) 0))
        (`self.HandleFirstTwoInBirthQuene`)))
    (:`then_2`
      (if (not (== (`KismetArrayLibrary.Array_Length` (`self.HuntQuene`)) 0))
        (`self.HandleFirstOneInHuntQuene`)))))

(event `GetAllSlimes`
  (bind _outactors (`GameplayStatics.GetAllActorsOfClass` "/Game/LianJiaCheng/Blueprint/Slime/BP_Slime_Parent.BP_Slime_Parent_C"))
  (set `self.AllSlimes` _outactors)
  (`KismetSystemLibrary.Delay` 1.0)
  (`self.GetAllSlimes`))

(fn `DoesSlimeShouldDie`
  (params (SlimeAttacked :type "Actor Object Reference") (SlimeAttacking :type "Actor Object Reference"))
  (returns (ShouldDie :type Boolean))
  (bind _asbp_slime_parent (cast `/Game/LianJiaCheng/Blueprint/Slime/BP_Slime_Parent` SlimeAttacked))
  (bind _asbp_slime_parent_2 (cast `/Game/LianJiaCheng/Blueprint/Slime/BP_Slime_Parent` SlimeAttacking))
  ;[1 1 1] Switch Situations
  (switch `/Game/LianJiaCheng/Blueprint/Slime/E_Slime_ClassNum` (`/Game/LianJiaCheng/Blueprint/Slime/BP_Slime_Parent.ClassEnum` _asbp_slime_parent)
    (:`NewEnumerator0`
      (bind _classenum (`/Game/LianJiaCheng/Blueprint/Slime/BP_Slime_Parent.ClassEnum` _asbp_slime_parent_2))
      (switch `/Game/LianJiaCheng/Blueprint/Slime/E_Slime_ClassNum` _classenum
        (:`NewEnumerator0`
          (set `self.TmpDeathRate` (`|GetArrayItem` (`self.DeathRateArray`))))
        (:`NewEnumerator1`
          (set `self.TmpDeathRate` (`|GetArrayItem` (`self.DeathRateArray`) 1)))
        (:`NewEnumerator2`
          (set `self.TmpDeathRate` (`|GetArrayItem` (`self.DeathRateArray`) 2)))
        (:`NewEnumerator3`
          (set `self.TmpDeathRate` (`|GetArrayItem` (`self.DeathRateArray`) 3)))))
    (:`NewEnumerator1`
      (switch `/Game/LianJiaCheng/Blueprint/Slime/E_Slime_ClassNum` _classenum
        (:`NewEnumerator0`
          (set `self.TmpDeathRate` (`|GetArrayItem` (`self.DeathRateArray`) 4)))
        (:`NewEnumerator1`
          (set `self.TmpDeathRate` (`|GetArrayItem` (`self.DeathRateArray`) 5)))
        (:`NewEnumerator2`
          (set `self.TmpDeathRate` (`|GetArrayItem` (`self.DeathRateArray`) 6)))
        (:`NewEnumerator3`
          (set `self.TmpDeathRate` (`|GetArrayItem` (`self.DeathRateArray`) 7)))))
    (:`NewEnumerator2`
      (switch `/Game/LianJiaCheng/Blueprint/Slime/E_Slime_ClassNum` _classenum
        (:`NewEnumerator0`
          (set `self.TmpDeathRate` (`|GetArrayItem` (`self.DeathRateArray`) 8)))
        (:`NewEnumerator1`
          (set `self.TmpDeathRate` (`|GetArrayItem` (`self.DeathRateArray`) 9)))
        (:`NewEnumerator2`
          (set `self.TmpDeathRate` (`|GetArrayItem` (`self.DeathRateArray`) 10)))
        (:`NewEnumerator3`
          (set `self.TmpDeathRate` (`|GetArrayItem` (`self.DeathRateArray`) 11)))))
    (:`NewEnumerator3`
      (switch `/Game/LianJiaCheng/Blueprint/Slime/E_Slime_ClassNum` _classenum
        (:`NewEnumerator0`
          (set `self.TmpDeathRate` (`|GetArrayItem` (`self.DeathRateArray`) 12)))
        (:`NewEnumerator1`
          (set `self.TmpDeathRate` (`|GetArrayItem` (`self.DeathRateArray`) 13)))
        (:`NewEnumerator2`
          (set `self.TmpDeathRate` (`|GetArrayItem` (`self.DeathRateArray`) 14)))
        (:`NewEnumerator3`
          (set `self.TmpDeathRate` (`|GetArrayItem` (`self.DeathRateArray`) 15))))))
  (if (< (`KismetMathLibrary.RandomFloatInRange` 0.0 100.0) (* (`self.TmpDeathRate`) 100.0))
    (return true)
    (else
      (return false))))

(fn `DoesSlimeShouldGiveBirth`
  (params (Mother1 :type "Actor Object Reference") (Mother2 :type "Actor Object Reference"))
  (returns (ShouldGiveBirth :type Boolean))
  (`/Engine/EditorBlueprintResources/StandardMacros.IsValid` Mother1
    (:`Is Valid`
      (`/Engine/EditorBlueprintResources/StandardMacros.IsValid` Mother2
        (:`Is Valid`
          (bind _asbp_slime_parent (cast `/Game/LianJiaCheng/Blueprint/Slime/BP_Slime_Parent` Mother1)
            (:`then`
              (bind _asbp_slime_parent_2 (cast `/Game/LianJiaCheng/Blueprint/Slime/BP_Slime_Parent` Mother2)
                (:`then`
                  ;[1 1 1] Switch Situations
                  (switch `/Game/LianJiaCheng/Blueprint/Slime/E_Slime_ClassNum` (`/Game/LianJiaCheng/Blueprint/Slime/BP_Slime_Parent.ClassEnum` _asbp_slime_parent)
                    (:`NewEnumerator0`
                      (bind _classenum (`/Game/LianJiaCheng/Blueprint/Slime/BP_Slime_Parent.ClassEnum` _asbp_slime_parent_2))
                      (switch `/Game/LianJiaCheng/Blueprint/Slime/E_Slime_ClassNum` _classenum
                        (:`NewEnumerator0`
                          (set `self.TmpBirthRate` (`|GetArrayItem` (`self.BirthHappenRateArray`))))
                        (:`NewEnumerator1`
                          (set `self.TmpBirthRate` (`|GetArrayItem` (`self.BirthHappenRateArray`) 1)))
                        (:`NewEnumerator2`
                          (set `self.TmpBirthRate` (`|GetArrayItem` (`self.BirthHappenRateArray`) 3)))
                        (:`NewEnumerator3`
                          (set `self.TmpBirthRate` (`|GetArrayItem` (`self.BirthHappenRateArray`) 6)))))
                    (:`NewEnumerator1`
                      (switch `/Game/LianJiaCheng/Blueprint/Slime/E_Slime_ClassNum` _classenum
                        (:`NewEnumerator0`
                          (set `self.TmpBirthRate` (`|GetArrayItem` (`self.BirthHappenRateArray`) 1)))
                        (:`NewEnumerator1`
                          (set `self.TmpBirthRate` (`|GetArrayItem` (`self.BirthHappenRateArray`) 2)))
                        (:`NewEnumerator2`
                          (set `self.TmpBirthRate` (`|GetArrayItem` (`self.BirthHappenRateArray`) 4)))
                        (:`NewEnumerator3`
                          (set `self.TmpBirthRate` (`|GetArrayItem` (`self.BirthHappenRateArray`) 7)))))
                    (:`NewEnumerator2`
                      (switch `/Game/LianJiaCheng/Blueprint/Slime/E_Slime_ClassNum` _classenum
                        (:`NewEnumerator0`
                          (set `self.TmpBirthRate` (`|GetArrayItem` (`self.BirthHappenRateArray`) 3)))
                        (:`NewEnumerator1`
                          (set `self.TmpBirthRate` (`|GetArrayItem` (`self.BirthHappenRateArray`) 4)))
                        (:`NewEnumerator2`
                          (set `self.TmpBirthRate` (`|GetArrayItem` (`self.BirthHappenRateArray`) 5)))
                        (:`NewEnumerator3`
                          (set `self.TmpBirthRate` (`|GetArrayItem` (`self.BirthHappenRateArray`) 8)))))
                    (:`NewEnumerator3`
                      (switch `/Game/LianJiaCheng/Blueprint/Slime/E_Slime_ClassNum` _classenum
                        (:`NewEnumerator0`
                          (set `self.TmpBirthRate` (`|GetArrayItem` (`self.BirthHappenRateArray`) 6)))
                        (:`NewEnumerator1`
                          (set `self.TmpBirthRate` (`|GetArrayItem` (`self.BirthHappenRateArray`) 7)))
                        (:`NewEnumerator2`
                          (set `self.TmpBirthRate` (`|GetArrayItem` (`self.BirthHappenRateArray`) 8)))
                        (:`NewEnumerator3`
                          (set `self.TmpBirthRate` 0.0)))))
                  (if (<= (`KismetMathLibrary.RandomFloatInRange` 0.0 100.0) (* (`self.TmpBirthRate`) 100.0))
                    (return true)
                    (else
                      (return false))))
                (:`CastFailed`
                  _)))
            (:`CastFailed`
              _)))
        (:`Is Not Valid`
          _)))
    (:`Is Not Valid`
      _))
  (return false))

(fn `FindNearistDifferentSideSlime`
  (params (Hunter :type "Actor Object Reference"))
  (bind _tmpprayindex (`self.TmpPrayIndex`))
  (bind _lasthitslimetoneglect (`self.LastHitSlimeToNeglect`))
  (set `self.TmpHunter` Hunter)
  (`|ExecutionSequence`
    (:`then_0`
      ;[1 1 1] Init
      (set `self.TmpHuntDis` 999999.0)
      (set `self.TmpPrayIndex` -1)
      (bind _asbp_slime_parent (cast `/Game/LianJiaCheng/Blueprint/Slime/BP_Slime_Parent` (`self.TmpHunter`)))
      (set `self.LastHitSlimeToNeglect` (`/Game/LianJiaCheng/Blueprint/Slime/BP_Slime_Parent.LastHitSlimeToNeglect` _asbp_slime_parent)))
    (:`then_1`
      ;[1 1 1] Is Slimes Array Empty?
      (if (!= (`KismetArrayLibrary.Array_Length` (`self.AllSlimes`)) 0)
        ;[1 1 1] Find Nearist Different Side Slime In World
        (for (_array_element _array_index) (`self.AllSlimes`)
          (`/Engine/EditorBlueprintResources/StandardMacros.IsValid` _lasthitslimetoneglect
            (:`Is Valid`
              (if (not (== _array_element _lasthitslimetoneglect))
                (bind _asbp_slime_parent_2 (cast `/Game/LianJiaCheng/Blueprint/Slime/BP_Slime_Parent` _array_element :!label _label))
                (`/Engine/EditorBlueprintResources/StandardMacros.IsValid` _asbp_slime_parent_2
                  (:`Is Valid`
                    (bind _asbp_slime_parent_3 (cast `/Game/LianJiaCheng/Blueprint/Slime/BP_Slime_Parent` (`self.TmpHunter`)))
                    (if (`|EnumInequality` (`/Game/LianJiaCheng/Blueprint/Slime/BP_Slime_Parent.SideEnum` _asbp_slime_parent_2) (`/Game/LianJiaCheng/Blueprint/Slime/BP_Slime_Parent.SideEnum` _asbp_slime_parent_3))
                      (bind _returnvalue (`self.GetDistanceTo` (`self.TmpHunter`) _asbp_slime_parent_2))
                      (if (> (`self.TmpHuntDis`) _returnvalue)
                        (set `self.TmpHuntDis` _returnvalue)
                        (set `self.TmpPrayIndex` _array_index)))))))
            (:`Is Not Valid`
              (goto _label))))
        ;[1 1 1] Return Slime Found
        (if (== _tmpprayindex -1)
          (bind _asbp_slime_parent_4 (cast `/Game/LianJiaCheng/Blueprint/Slime/BP_Slime_Parent` (`self.TmpHunter`)))
          (set `/Game/LianJiaCheng/Blueprint/Slime/BP_Slime_Parent.Pary` null _asbp_slime_parent_4)
          (else
            (bind _asbp_slime_parent_5 (cast `/Game/LianJiaCheng/Blueprint/Slime/BP_Slime_Parent` (`self.TmpHunter`)))
            (set `/Game/LianJiaCheng/Blueprint/Slime/BP_Slime_Parent.Pary` (`|GetArrayItem` (`self.AllSlimes`) _tmpprayindex) _asbp_slime_parent_5)))))))

(fn `FindNearistSameSideFemaleSlime`
  (params (Hunter :type "Actor Object Reference"))
  (bind _tmpprayindex (`self.TmpPrayIndex`))
  (bind _lasthitslimetoneglect (`self.LastHitSlimeToNeglect`))
  (set `self.TmpHunter` Hunter)
  (`|ExecutionSequence`
    (:`then_0`
      ;[1 1 1] Init
      (set `self.TmpHuntDis` 999999.0)
      (set `self.TmpPrayIndex` -1)
      (bind _asbp_slime_parent (cast `/Game/LianJiaCheng/Blueprint/Slime/BP_Slime_Parent` (`self.TmpHunter`)))
      (set `self.LastHitSlimeToNeglect` (`/Game/LianJiaCheng/Blueprint/Slime/BP_Slime_Parent.LastHitSlimeToNeglect` _asbp_slime_parent)))
    (:`then_1`
      ;[1 1 1] Is Slimes Array Empty?
      (if (!= (`KismetArrayLibrary.Array_Length` (`self.AllSlimes`)) 0)
        ;[1 1 1] Find Nearist Different Side Slime In World
        (for (_array_element _array_index) (`self.AllSlimes`)
          (set `self.TmpPary` _array_element)
          ;;[1 1 1] Should TmpPary be neglect?
          (`/Engine/EditorBlueprintResources/StandardMacros.IsValid` _lasthitslimetoneglect
            (:`Is Valid`
              (if (not (== (`self.TmpPary`) _lasthitslimetoneglect))
                ;;[1 1 1] Is TmpPary == TmpHunter?
                (if (not (== (`self.TmpPary`) (`self.TmpHunter`))) :!label _label
                  (bind _asbp_slime_parent_2 (cast `/Game/LianJiaCheng/Blueprint/Slime/BP_Slime_Parent` (`self.TmpPary`)))
                  (`/Engine/EditorBlueprintResources/StandardMacros.IsValid` _asbp_slime_parent_2
                    (:`Is Valid`
                      (bind _asbp_slime_parent_3 (cast `/Game/LianJiaCheng/Blueprint/Slime/BP_Slime_Parent` (`self.TmpHunter`)))
                      ;;[1 1 1] Is TmpPary In Birth Delay
                      (if (not (`/Game/LianJiaCheng/Blueprint/Slime/BP_Slime_Parent.IsBirthDelay` _asbp_slime_parent_2))
                        (bind _classenum (`/Game/LianJiaCheng/Blueprint/Slime/BP_Slime_Parent.ClassEnum` _asbp_slime_parent_2))
                        ;;[1 1 1] Is TmpPary Female And Same Side with TmpHunter?
                        (if (or (`|EnumEquality` _classenum "NewEnumerator2") (`|EnumEquality` _classenum "NewEnumerator3"))
                          (if (`|EnumEquality` (`/Game/LianJiaCheng/Blueprint/Slime/BP_Slime_Parent.SideEnum` _asbp_slime_parent_2) (`/Game/LianJiaCheng/Blueprint/Slime/BP_Slime_Parent.SideEnum` _asbp_slime_parent_3))
                            (bind _returnvalue (`self.GetDistanceTo` (`self.TmpHunter`) _asbp_slime_parent_2))
                            ;;[1 1 1] Is TmpPary nearer?
                            (if (> (`self.TmpHuntDis`) _returnvalue)
                              ;;[1 1 1] Find TmpPary Nearer
                              (set `self.TmpHuntDis` _returnvalue)
                              (set `self.TmpPrayIndex` _array_index))))))))))
            (:`Is Not Valid`
              (goto _label))))
        ;[1 1 1] Return Slime Found
        (if (== _tmpprayindex -1)
          (bind _asbp_slime_parent_4 (cast `/Game/LianJiaCheng/Blueprint/Slime/BP_Slime_Parent` (`self.TmpHunter`)))
          (set `/Game/LianJiaCheng/Blueprint/Slime/BP_Slime_Parent.Pary` null _asbp_slime_parent_4)
          (else
            (bind _asbp_slime_parent_5 (cast `/Game/LianJiaCheng/Blueprint/Slime/BP_Slime_Parent` (`self.TmpHunter`)))
            (set `/Game/LianJiaCheng/Blueprint/Slime/BP_Slime_Parent.Pary` (`|GetArrayItem` (`self.AllSlimes`) _tmpprayindex) _asbp_slime_parent_5)))))))

(fn `HandleFirstOneInHuntQuene`
  (bind _output (`|GetArrayItem` (`self.HuntQuene`)))
  ;[1 1 1] IsObjValid?
  (`/Engine/EditorBlueprintResources/StandardMacros.IsValid` _output
    (:`Is Valid`
      (`|ExecutionSequence`
        (:`then_0`
          (bind _asbp_slime_parent (cast `/Game/LianJiaCheng/Blueprint/Slime/BP_Slime_Parent` _output))
          (switch `/Game/LianJiaCheng/Blueprint/Slime/E_Slime_ClassNum` (`/Game/LianJiaCheng/Blueprint/Slime/BP_Slime_Parent.ClassEnum` _asbp_slime_parent)
            (:`NewEnumerator0`
              (`self.FindNearistDifferentSideSlime` _output))
            (:`NewEnumerator1`
              (`self.FindNearistDifferentSideSlime` _output))
            (:`NewEnumerator2`
              (`self.FindNearistSameSideFemaleSlime` _output))
            (:`NewEnumerator3`
              (`self.FindNearistSameSideFemaleSlime` _output))))
        (:`then_1`
          ;[1 1 1] End
          (`KismetArrayLibrary.Array_Remove` (`self.HuntQuene`) :!label _label))))
    (:`Is Not Valid`
      (goto _label))))

(fn `HandleFirstTwoInBirthQuene`
  (bind _inputreadyquene2 (`self.InputReadyQuene2`))
  (bind _inputreadyquene2_2 (`self.InputReadyQuene2`))
  (bind _inputreadyquene2_3 (`self.InputReadyQuene2`))
  (bind _inputreadyquene2_4 (`self.InputReadyQuene2`))
  ;[1 1 1] There is No Need To Worry About "TryGiveBirth" is Called Twice Because the First Call will Set "IsBirthDelay" and the second Call will Break
  (bind _isbothfalse (`self.IsBothBirthDelayFalse` (`|GetArrayItem` _inputreadyquene2) (`|GetArrayItem` _inputreadyquene2 1)))
  (if _isbothfalse
    ;[1 1 1] ShouldGiveBirth?
    (bind _shouldgivebirth (`self.DoesSlimeShouldGiveBirth` (`|GetArrayItem` _inputreadyquene2_2) (`|GetArrayItem` _inputreadyquene2_2 1)))
    (if _shouldgivebirth
      ;[1 1 1] Set CD After GiveBirth
      (bind _asbp_slime_parent (cast `/Game/LianJiaCheng/Blueprint/Slime/BP_Slime_Parent` (`|GetArrayItem` _inputreadyquene2_3))
        (:`then`
          (bind _asbp_slime_parent_2 (cast `/Game/LianJiaCheng/Blueprint/Slime/BP_Slime_Parent` (`|GetArrayItem` _inputreadyquene2_3 1))
            (:`then`
              ;;[1 1 1] JoinInBirth
              (`/Game/LianJiaCheng/Blueprint/Slime/BP_Slime_Parent.JoinInBirth` _asbp_slime_parent)
              (`/Game/LianJiaCheng/Blueprint/Slime/BP_Slime_Parent.JoinInBirth` _asbp_slime_parent_2)
              ;[1 0 0] GiveBirth
              (bind _asbp_slime_parent_3 (cast `/Game/LianJiaCheng/Blueprint/Slime/BP_Slime_Parent` (`|GetArrayItem` (`self.InputReadyQuene2`)))
                (:`then`
                  (`/Game/LianJiaCheng/Blueprint/Slime/BP_Slime_Parent.GiveBirth` _asbp_slime_parent_3))
                (:`CastFailed`
                  _)))
            (:`CastFailed`
              _)))
        (:`CastFailed`
          _))))
  ;[1 1 1] End
  (`KismetArrayLibrary.Array_Remove` _inputreadyquene2_4)
  (`KismetArrayLibrary.Array_Remove` _inputreadyquene2_4))

(fn `HandleFirstTwoInDeathQuene`
  (bind _inputreadyquene1 (`self.InputReadyQuene1`))
  (bind _inputreadyquene1_2 (`self.InputReadyQuene1`))
  (bind _inputreadyquene1_3 (`self.InputReadyQuene1`))
  (bind _inputreadyquene1_4 (`self.InputReadyQuene1`))
  ;[1 1 1] IsObjValid?
  (`/Engine/EditorBlueprintResources/StandardMacros.IsValid` (`|GetArrayItem` _inputreadyquene1_2)
    (:`Is Valid`
      (`/Engine/EditorBlueprintResources/StandardMacros.IsValid` (`|GetArrayItem` _inputreadyquene1_2 1)
        (:`Is Valid`
          (`|ExecutionSequence`
            (:`then_0`
              ;[1 1 1] Clear SlimeToDie
              (`KismetArrayLibrary.Array_Clear` (`self.SlimeToDie`)))
            (:`then_1`
              ;[1 1 1] Init Slime1 Situation
              (bind _asbp_slime_parent (cast `/Game/LianJiaCheng/Blueprint/Slime/BP_Slime_Parent` (`|GetArrayItem` _inputreadyquene1_3)))
              (bind _asbp_slime_parent_2 (cast `/Game/LianJiaCheng/Blueprint/Slime/BP_Slime_Parent` (`|GetArrayItem` _inputreadyquene1_3 1)))
              (bind _output_get (set `self.SilmeAttacked` _asbp_slime_parent))
              (bind _output_get_2 (set `self.SlimeAttacking` _asbp_slime_parent_2))
              (bind _shoulddie (`self.DoesSlimeShouldDie` _output_get _output_get_2))
              (if _shoulddie
                (`KismetArrayLibrary.Array_Add` (`self.SlimeToDie`) (`self.SilmeAttacked`))))
            (:`then_2`
              ;[1 1 1] Init Slime2 Situation
              (bind _asbp_slime_parent_3 (cast `/Game/LianJiaCheng/Blueprint/Slime/BP_Slime_Parent` (`|GetArrayItem` _inputreadyquene1_4 1)))
              (bind _asbp_slime_parent_4 (cast `/Game/LianJiaCheng/Blueprint/Slime/BP_Slime_Parent` (`|GetArrayItem` _inputreadyquene1_4)))
              (bind _output_get_3 (set `self.SilmeAttacked` _asbp_slime_parent_3))
              (bind _output_get_4 (set `self.SlimeAttacking` _asbp_slime_parent_4))
              (bind _shoulddie_2 (`self.DoesSlimeShouldDie` _output_get_3 _output_get_4))
              (if _shoulddie_2
                (`KismetArrayLibrary.Array_Add` (`self.SlimeToDie`) (`self.SilmeAttacked`))))
            (:`then_3`
              ;[1 0 0] Die
              (for _array_element (`self.SlimeToDie`)
                (`/Engine/EditorBlueprintResources/StandardMacros.IsValid` _array_element
                  (:`Is Valid`
                    (`/Game/LianJiaCheng/Blueprint/Slime/BP_Slime_Parent.Die` _array_element "NewEnumerator0")))))
            (:`then_4`
              ;[1 1 1] End
              (`KismetArrayLibrary.Array_Remove` _inputreadyquene1 :!label _label)
              (`KismetArrayLibrary.Array_Remove` _inputreadyquene1))))
        (:`Is Not Valid`
          (goto _label))))
    (:`Is Not Valid`
      (goto _label))))

(fn `IsBothBirthDelayFalse`
  (params (Mother1 :type "Actor Object Reference") (Mother2 :type "Actor Object Reference"))
  (returns (IsBothFalse :type Boolean))
  (`/Engine/EditorBlueprintResources/StandardMacros.IsValid` Mother1
    (:`Is Valid`
      (`/Engine/EditorBlueprintResources/StandardMacros.IsValid` Mother2
        (:`Is Valid`
          (bind _asbp_slime_parent (cast `/Game/LianJiaCheng/Blueprint/Slime/BP_Slime_Parent` Mother1)
            (:`then`
              (bind _asbp_slime_parent_2 (cast `/Game/LianJiaCheng/Blueprint/Slime/BP_Slime_Parent` Mother2)
                (:`then`
                  ;[1 1 1] IsBirthDelay?
                  (if (and (== (`/Game/LianJiaCheng/Blueprint/Slime/BP_Slime_Parent.IsBirthDelay` _asbp_slime_parent) false) (== (`/Game/LianJiaCheng/Blueprint/Slime/BP_Slime_Parent.IsBirthDelay` _asbp_slime_parent_2) false))
                    (return true)
                    (else
                      (return false))))
                (:`CastFailed`
                  _)))
            (:`CastFailed`
              _)))
        (:`Is Not Valid`
          _)))
    (:`Is Not Valid`
      _))
  (return false))

(fn `UserConstructionScript`)