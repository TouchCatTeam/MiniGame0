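; BP_Slime_Parent is the base slime actor, belonging to a side and able to breed or fight on contact with other slimes.
; After a short delay, hits report to the BP_Judgment actor's birth queue for same-side slimes or death queue for opposing ones.
; Die and born events toggle visibility and collision rather than destroying or spawning, alongside a timed birth-cooldown flag.
; A view sphere tracks nearby same-side slimes, and BeginPlay records the walking centre.
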(event `self.ReceiveBeginPlay`
  ;[1 1 1] Walk Init
  (`SphereComponent.SetSphereRadius` (`self.ViewSphere`) (`self.ViewSphereRadius`) true)
  (set `self.WalkingCentre ` (`self.K2_GetActorLocation` self)))

(event `self.ReceiveHit`
  (params (MyComp :type "PrimitiveComponent Object Reference") (Other :type "Actor Object Reference") (OtherComp :type "PrimitiveComponent Object Reference") (bSelfMoved :type Boolean) (HitLocation :type "Vector Structure") (HitNormal :type "Vector Structure") (NormalImpulse :type "Vector Structure") (Hit :type "HitResult Structure (by ref)"))
  (bind _otheractor (`self.OtherActor`))
  ;[1 1 1] Hit Event
  ;;[1 1 1] Only Consider: One Shared Parent
  (bind _output_get (set `self.OtherActor` Other))
  (bind _asbp_slime_parent (cast `/Game/LianJiaCheng/Blueprint/Slime/BP_Slime_Parent` _output_get))
  ;;[1 1 1] DeathOrBirth
  (if (`|EnumEquality` (`/Game/LianJiaCheng/Blueprint/Slime/BP_Slime_Parent.SideEnum` _asbp_slime_parent) (`self.SideEnum`))
    (`KismetSystemLibrary.Delay` 0.2)
    (bind _outactors (`GameplayStatics.GetAllActorsOfClass` "/Game/LianJiaCheng/Blueprint/Judgment/BP_Judgment.BP_Judgment_C"))
    (message `/Game/LianJiaCheng/Blueprint/Judgment/BPI_Judgment.AddBirthQuene` (`|GetArrayItem` _outactors) self _otheractor)
    (else
      (`KismetSystemLibrary.Delay` 0.2)
      (bind _outactors_2 (`GameplayStatics.GetAllActorsOfClass` "/Game/LianJiaCheng/Blueprint/Judgment/BP_Judgment.BP_Judgment_C"))
      (message `/Game/LianJiaCheng/Blueprint/Judgment/BPI_Judgment.AddDeathQuene` (`|GetArrayItem` _outactors_2) self _otheractor))))

(event `JoinInBirth`
  ;[1 1 1] BirthDelay
  (set `self.IsBirthDelay` true)
  (`KismetSystemLibrary.Delay` (`self.BirthDelayTime`))
  (set `self.IsBirthDelay` false))

(event `Die Event`
  (`self.SetActorHiddenInGame` true)
  (`self.SetActorEnableCollision` false))

(event `Born Event`
  (`self.SetActorHiddenInGame` false)
  (`self.SetActorEnableCollision` true))

(event `self.ViewSphere.OnComponentBeginOverlap`
  (params (OverlappedComponent :type "PrimitiveComponent Object Reference") (OtherActor :type "Actor Object Reference") (OtherComp :type "PrimitiveComponent Object Reference") (OtherBodyIndex :type Integer) (bFromSweep :type Boolean) (SweepResult :type "HitResult Structure (by ref)"))
  (bind _slimesspotted_ (`self.SlimesSpotted `))
  (bind _asbp_slime_parent (cast `/Game/LianJiaCheng/Blueprint/Slime/BP_Slime_Parent` OtherActor))
  ;[1 1 1] Allow Slime Different Side to Self
  (if (`|EnumEquality` (`/Game/LianJiaCheng/Blueprint/Slime/BP_Slime_Parent.SideEnum` _asbp_slime_parent) (`self.SideEnum`))
    ;[1 1 1] Allow Slime Different to Array
    (if (not (or (`KismetArrayLibrary.Array_Contains` _slimesspotted_ _asbp_slime_parent) (== _asbp_slime_parent self)))
      (`KismetArrayLibrary.Array_Add` _slimesspotted_ _asbp_slime_parent))))

(event `self.ViewSphere.OnComponentEndOverlap`
  (params (OverlappedComponent :type "PrimitiveComponent Object Reference") (OtherActor :type "Actor Object Reference") (OtherComp :type "PrimitiveComponent Object Reference") (OtherBodyIndex :type Integer))
  (bind _slimesspotted_ (`self.SlimesSpotted `))
  (bind _asbp_slime_parent (cast `/Game/LianJiaCheng/Blueprint/Slime/BP_Slime_Parent` OtherActor))
  ;[1 1 1] Allow Slime Different to Array
  (if (and (`KismetArrayLibrary.Array_Contains` _slimesspotted_ _asbp_slime_parent) (!= _asbp_slime_parent self))
    (`KismetArrayLibrary.Array_RemoveItem` _slimesspotted_ _asbp_slime_parent)))

(fn `UserConstructionScript`)