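; Prairie Fire cue actor that creates a timed area of fire which burns slimes.
; A sphere's overlap events track the slimes in range; StartFire resizes it, calls GetBurnt on those slimes and spawns a fire particle scaled to the radius.
; Slimes entering while it burns also get burnt and receive the explosion radius.
; After Duration, the particle and actor are destroyed.
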(event `StartFire`
  (params (FireEffectRadius :type "Float (double-precision)" :default 350.0) (ExplosionEffectRadius :type "Float (double-precision)" :default 300.0))
  (`|ExecutionSequence`
    (:`then_0`
      ;[1 1 1] Init
      (set `self.IsFire` true)
      (`SphereComponent.SetSphereRadius` (`self.Sphere`) FireEffectRadius true))
    (:`then_1`
      ;[1 1 1] Give Event to Slimes that has being in range
      (for _array_element (`self.SlimesInRange`)
        (bind _asbp_slime_parent (cast `/Game/LianJiaCheng/Blueprint/Slime/BP_Slime_Parent` _array_element))
        (`/Game/LianJiaCheng/Blueprint/Slime/BP_Slime_Parent.GetBurnt` _asbp_slime_parent ExplosionEffectRadius)))
    (:`then_2`
      ;[1 1 1] Comment
      (bind _returnvalue (`GameplayStatics.SpawnEmitterAtLocation` "/Game/LianJiaCheng/Effect/MagicCircles2/ParticleSystems/PS_PrairieFire.PS_PrairieFire" (+ (`self.K2_GetActorLocation` self) (`KismetMathLibrary.MakeVector` 0.0 0.0 10.0)) (struct) (`KismetMathLibrary.Conv_DoubleToVector` (/ FireEffectRadius (`self.EffectOriginalRadius`)))))
      (set `self.ParticleSystemToPlay` _returnvalue))
    (:`then_3`
      ;[1 1 1] End
      (`KismetSystemLibrary.Delay` (`self.Duration`))
      (`ActorComponent.K2_DestroyComponent` (`self.ParticleSystemToPlay`))
      (`self.K2_DestroyActor`))))

(event `self.Sphere.OnComponentBeginOverlap`
  (params (OverlappedComponent :type "PrimitiveComponent Object Reference") (OtherActor :type "Actor Object Reference") (OtherComp :type "PrimitiveComponent Object Reference") (OtherBodyIndex :type Integer) (bFromSweep :type Boolean) (SweepResult :type "HitResult Structure (by ref)"))
  ;[1 1 1] Ger Slimes In Range
  (bind _asbp_slime_parent (cast `/Game/LianJiaCheng/Blueprint/Slime/BP_Slime_Parent` OtherActor))
  (`KismetArrayLibrary.Array_Add` (`self.SlimesInRange`) _asbp_slime_parent)
  ;[1 1 1] Get Event to Slime that go into sphere
  (if (`self.IsFire`)
    (set `/Game/LianJiaCheng/Blueprint/Slime/BP_Slime_Parent.FireExplosionEffectRadius` (stale `StartFire` ExplosionEffectRadius) _asbp_slime_parent)
    (`/Game/LianJiaCheng/Blueprint/Slime/BP_Slime_Parent.GetBurnt` _asbp_slime_parent (stale `StartFire` ExplosionEffectRadius))))

(event `self.Sphere.OnComponentEndOverlap`
  (params (OverlappedComponent :type "PrimitiveComponent Object Reference") (OtherActor :type "Actor Object Reference") (OtherComp :type "PrimitiveComponent Object Reference") (OtherBodyIndex :type Integer))
  ;[1 1 1] Ger Slimes In Range
  (bind _asbp_slime_parent (cast `/Game/LianJiaCheng/Blueprint/Slime/BP_Slime_Parent` OtherActor))
  (`KismetArrayLibrary.Array_RemoveItem` (`self.SlimesInRange`) _asbp_slime_parent))

(fn `UserConstructionScript`)