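; Powerful Wind card effect actor that blows slimes along a wind path for a timed duration, then destroys itself.
; StartWind stores the path and spawns scaled Niagara tornado and updraft effects, looping in sound fades and camera shake.
; Tick launches slimes near the path line along it with cone jitter, randomly pulling others toward its start.
; Cleanup removes effects, lightens the sky and clears slimes' in-air flags.
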(event `self.ReceiveTick`
  (params (DeltaSeconds :type "Float (single-precision)"))
  (if (`self.IsWind`)
    (bind _outactors (`GameplayStatics.GetAllActorsOfClass` "/Game/LianJiaCheng/Blueprint/Slime/BP_Slime_Parent.BP_Slime_Parent_C"))
    (for _array_element _outactors
      (bind _asbp_slime_parent (cast `/Game/LianJiaCheng/Blueprint/Slime/BP_Slime_Parent` _array_element))
      ;[1 1 1] CanBlow
      (if (< (`KismetMathLibrary.VSize` (`KismetMathLibrary.Cross_VectorVector` (- (`self.K2_GetActorLocation` _asbp_slime_parent) (`self.WindStartPos`)) (`KismetMathLibrary.Normal` (- (`self.WindEndPos`) (`self.WindStartPos`))))) (`self.WindWidth`))
        ;[1 1 1] Apply Wind
        ;;[1 1 1] Blow Slime
        (`Character.LaunchCharacter` _asbp_slime_parent (* (+ (* (`KismetMathLibrary.GetUpVector` (struct)) 1.0) (`KismetMathLibrary.RandomUnitVectorInConeInDegrees` (`self.WindMainDir`) 30.0)) (`self.WindBlowVelocity`)) false false)
        (else
          ;;[1 1 1] Take in Velocity
          (if (< (`KismetMathLibrary.RandomFloatInRange` 0.0 1000.0) 90.0)
            (`Character.LaunchCharacter` _asbp_slime_parent (* (+ (* (`KismetMathLibrary.GetUpVector` (struct)) 0.5) (`KismetMathLibrary.RandomUnitVectorInConeInDegrees` (`KismetMathLibrary.Normal` (- (`self.WindStartPos`) (`self.K2_GetActorLocation` _asbp_slime_parent))) 30.0)) (`self.WindTakeInVelocity`)) false false)))))))

(event `StartWind`
  (params (WindStartPos :type "Vector Structure") (WindEndPos :type "Vector Structure") (WindEffectRadius :type "Float (double-precision)") (BlackCloud :type "ParticleSystemComponent Object Reference"))
  ;[1 1 1] Init Variable
  (set `self.WindStartPos` WindStartPos)
  (set `self.WindEndPos` WindEndPos)
  (set `self.WindEffectRadius` WindEffectRadius)
  (set `self.BlackCloudEffect` BlackCloud)
  (`|ExecutionSequence`
    (:`then_0`
      ;[1 1 1] Init
      (set `self.WindMainDir` (- (`self.WindEndPos`) (`self.WindStartPos`))))
    (:`then_1`
      ;[1 1 1] Wind Start
      (set `self.IsWind` true))
    (:`then_2`
      ;[1 1 1] Spawn Effect
      (bind _returnvalue (`NiagaraFunctionLibrary.SpawnSystemAtLocation` "/Game/LianJiaCheng/Effect/VFX_Wind_Pack/VFX_Niagara/NS_Wind_Tornado.NS_Wind_Tornado" (`self.WindStartPos`) (struct) (`KismetMathLibrary.Conv_DoubleToVector` (/ (`self.WindEffectRadius`) (`self.WindTornadoOriginalRadius`)))))
      (set `self.WindTornadoEffect` _returnvalue)
      (bind _returnvalue_2 (`NiagaraFunctionLibrary.SpawnSystemAtLocation` "/Game/LianJiaCheng/Effect/VFX_Wind_Pack/VFX_Niagara/NS_WindUpdraft.NS_WindUpdraft" (`self.WindStartPos`) (`KismetMathLibrary.ComposeRotators` (`KismetMathLibrary.MakeRotator` (.yaw (`KismetMathLibrary.FindLookAtRotation` (`self.WindStartPos`) (`self.WindEndPos`)))) (`KismetMathLibrary.MakeRotator` 0.0 -90.0)) (`KismetMathLibrary.Conv_DoubleToVector` (/ (`self.WindEffectRadius`) (`self.WindUpdraftOriginalRadius`)))))
      (set `self.WindUpdraftEffect` _returnvalue_2)
      ;[1 1 1] Spawn WindTornado Sound
      (bind _returnvalue_3 (`GameplayStatics.SpawnSound2D` "/Game/LianJiaCheng/Sound/S_PowfulWind_Blowing.S_PowfulWind_Blowing" 1.0 1.0 0.0 null))
      (bind _output_get (set `self.WindTornadoSound` _returnvalue_3))
      (`AudioComponent.FadeIn` _output_get (`self.WindTornadoSoundFadeInDuration`) 1.0 0.0 "Linear")
      ;[1 1 1] Play Camera Shake
      (`GameplayStatics.PlayWorldCameraShake` "/Game/LianJiaCheng/Effect/BP_CameraShake_WindTornado.BP_CameraShake_WindTornado_C" (`self.K2_GetActorLocation` (`GameplayStatics.GetPlayerCameraManager` 0)) 10.0 100.0))
    (:`then_3`
      ;[1 1 1] Wind Duration
      (`KismetSystemLibrary.Delay` (`self.WindTornadoEffectDuration`))
      ;[1 1 1] End WindTornado Sound
      (`AudioComponent.FadeOut` (`self.WindTornadoSound`) (`self.WindTornadoSoundFadeOutDuration`) 0.0 "Linear")
      (`KismetSystemLibrary.Delay` 1.0)
      (`|ExecutionSequence`
        (:`then_0`
          ;[1 1 1] End Wind Effect
          (`ActorComponent.K2_DestroyComponent` (`self.WindTornadoEffect`))
          (`ActorComponent.K2_DestroyComponent` (`self.WindUpdraftEffect`))
          (`ActorComponent.K2_DestroyComponent` (`self.BlackCloudEffect`)))
        (:`then_1`
          ;[1 1 1] Stop Camera Shake
          (`PlayerCameraManager.StopAllCameraShakes` (`GameplayStatics.GetPlayerCameraManager` 0) true))
        (:`then_2`
          ;[1 1 1] PPV
          (bind _returnvalue_4 (`GameplayStatics.GetActorOfClass` "/Game/LianJiaCheng/Blueprint/Card/BP_CardRepertory.BP_CardRepertory_C"))
          (`/Game/LianJiaCheng/Blueprint/Card/BP_CardRepertory.SkyLighten` _returnvalue_4))
        (:`then_3`
          ;[1 1 1] End Wind Blow
          (set `self.IsWind` false)
          ;;[1 1 1] IsAir
          (bind _outactors (`GameplayStatics.GetAllActorsOfClass` "/Game/LianJiaCheng/Blueprint/Slime/BP_Slime_Parent.BP_Slime_Parent_C"))
          (for _array_element _outactors
            (bind _asbp_slime_parent (cast `/Game/LianJiaCheng/Blueprint/Slime/BP_Slime_Parent` _array_element))
            (set `/Game/LianJiaCheng/Blueprint/Slime/BP_Slime_Parent.IsInAir` false _asbp_slime_parent))
          ;[1 1 1] End Actor
          (`self.K2_DestroyActor`))))))

(fn `UserConstructionScript`
  ;[1 1 1] Get Judger
  (bind _outactors (`GameplayStatics.GetAllActorsOfClass` "/Game/LianJiaCheng/Blueprint/Judger/BP_Judger.BP_Judger_C"))
  (set `self.Judger` (`|GetArrayItem` _outactors)))