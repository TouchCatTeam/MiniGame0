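; Card effect repertory actor that runs the targeting and casting of six slime-game cards, from PrairieFire to SlimeCreeper.
; CardEffectHandler routes card and use state to per-card functions that spawn indicators, then GamePlayCue actors on confirm.
; Tick aims PowerfulWind's second-step arrow decal at the cursor and marks SlimeCreeper's candidate slime in red.
; Some cards darken the sky by timeline-blending two tagged post-process volumes; only PowerfulWind's cancel reverses it here.
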(event `self.ReceiveBeginPlay`
  ;[1 1 1] Get PPV
  (`|ExecutionSequence`
    (:`then_0`
      (bind _outactors (`GameplayStatics.GetAllActorsWithTag` "DarkPPV"))
      (bind _aspost_process_volume (cast `PostProcessVolume` (`|GetArrayItem` _outactors)))
      (set `self.DarkPPV` _aspost_process_volume))
    (:`then_1`
      (bind _outactors_2 (`GameplayStatics.GetAllActorsWithTag` "MainPPV"))
      (bind _aspost_process_volume_2 (cast `PostProcessVolume` (`|GetArrayItem` _outactors_2)))
      (set `self.MainPPV` _aspost_process_volume_2))))

(event `SkyDarken`
  (bind (_direction _alpha) (`Timeline|DarkTimeline` :!label _label)
    (:`Update`
      (set `PostProcessVolume.BlendWeight` (`KismetMathLibrary.Lerp` 0.0 0.4 _alpha) (`self.DarkPPV`))
      (set `PostProcessVolume.BlendWeight` (`KismetMathLibrary.Lerp` 1.0 0.0 _alpha) (`self.MainPPV`)))))

(event `SkyLighten`
  (goto _label :!via `Reverse`))

(event `self.ReceiveTick`
  (params (DeltaSeconds :type "Float (single-precision)"))
  (bind _tmpchosencreeper (`self.TmpChosenCreeper`))
  (bind _tmpchosencreeper_2 (`self.TmpChosenCreeper`))
  (bind _tmpchosencreeper_3 (`self.TmpChosenCreeper`))
  (bind _tmpindicator1 (`self.TmpIndicator1`))
  (bind _tmpchosencreeperindicator (`self.TmpChosenCreeperIndicator`))
  (bind _tmpchosencreeperindicator_2 (`self.TmpChosenCreeperIndicator`))
  (`|ExecutionSequence`
    (:`then_0`
      ;[1 1 1] PowerfulWind
      (if (`self.IsWinding`)
        (`/Engine/EditorBlueprintResources/StandardMacros.IsValid` (`self.TmpWindDecal2`)
          (:`Is Valid`
            (bind (_hitactor _location) (`self.GetMouseHit`))
            (`|ExecutionSequence`
              (:`then_0`
                (bind _yaw (.yaw (`KismetMathLibrary.FindLookAtRotation` (`SceneComponent.K2_GetComponentLocation` (`self.TmpDecal1`)) _location)))
                ;;[1 1 1] Update Wind2 Decal Rot
                (`SceneComponent.K2_SetWorldRotation` (`self.TmpWindDecal2`) (`KismetMathLibrary.MakeRotator` 0.0 -90.0 _yaw) false false))
              (:`then_1`
                ;;[1 1 1] Update Wind2Decal Pos
                (`SceneComponent.K2_SetWorldLocation` (`self.TmpWindDecal2`) (+ (- _location (* (`KismetMathLibrary.GetForwardVector` (`KismetMathLibrary.MakeRotator` 0.0 0.0 _yaw)) (`self.WindArrowIndicatorRadius`))) (`KismetMathLibrary.MakeVector` 0.0 0.0 50.0)) false false)))))))
    (:`then_1`
      ;[1 1 1] Creeper
      ;;[1 1 1] Is Choosing Creeper?
      (if (`self.IsChoosingCreeper`)
        (`|ExecutionSequence`
          (:`then_0`
            ;;[1 1 1] Have Indicator?
            (`/Engine/EditorBlueprintResources/StandardMacros.IsValid` _tmpindicator1
              (:`Is Valid`
                (bind _asbp_dot_indicator (cast `/Game/LianJiaCheng/Blueprint/Card/BP_DotIndicator` _tmpindicator1))
                (bind _slimesinrange (`/Game/LianJiaCheng/Blueprint/Card/BP_DotIndicator.SlimesInRange` _asbp_dot_indicator))
                ;;[1 1 1] Get(Update) Creeper Chosen By Indicator
                (if (> (`KismetArrayLibrary.Array_Length` _slimesinrange) 0)
                  (set `self.TmpChosenCreeper` (`|GetArrayItem` _slimesinrange))
                  ;;[1 1 1] Hasnt Spawn Chosen Creeper Indicator: Spawn New Indicator
                  (`/Engine/EditorBlueprintResources/StandardMacros.IsValid` (`self.TmpChosenCreeperIndicator`)
                    (:`Is Valid`
                      ;;[1 1 1] Refresh Indicator
                      (`/Engine/EditorBlueprintResources/StandardMacros.IsValid` _tmpchosencreeper_3
                        (:`Is Valid`
                          (bind _asbp_slime_parent (cast `/Game/LianJiaCheng/Blueprint/Slime/BP_Slime_Parent` _tmpchosencreeper_3))
                          (bind _asbp_dot_indicator_2 (cast `/Game/LianJiaCheng/Blueprint/Card/BP_DotIndicator` (`self.TmpChosenCreeperIndicator`)))
                          (`/Game/LianJiaCheng/Blueprint/Card/BP_DotIndicator.InitDecal` _asbp_dot_indicator_2 (* (`SphereComponent.SphereRadius` (`/Game/LianJiaCheng/Blueprint/Slime/BP_Slime_Parent.IdentitySphere` _asbp_slime_parent)) 3.0) false))))
                    (:`Is Not Valid`
                      (`/Engine/EditorBlueprintResources/StandardMacros.IsValid` _tmpchosencreeper_2
                        (:`Is Valid`
                          (bind _returnvalue (`|SpawnActorFromClass` "/Game/LianJiaCheng/Blueprint/Card/BP_DotIndicator.BP_DotIndicator_C" (`KismetMathLibrary.Conv_VectorToTransform` (`self.K2_GetActorLocation` _tmpchosencreeper_2)) "Undefined" "OverrideRootScale" null null))
                          ;;[1 1 1] Init Indicator
                          (bind _asbp_slime_parent_2 (cast `/Game/LianJiaCheng/Blueprint/Slime/BP_Slime_Parent` _tmpchosencreeper_2))
                          (`/Game/LianJiaCheng/Blueprint/Card/BP_DotIndicator.InitDecal` _returnvalue (* (`SphereComponent.SphereRadius` (`/Game/LianJiaCheng/Blueprint/Slime/BP_Slime_Parent.IdentitySphere` _asbp_slime_parent_2)) 3.0) false)
                          (set `self.TmpChosenCreeperIndicator` _returnvalue)
                          ;;[1 1 1] Set Red Color
                          (bind _returnvalue_2 (`DecalComponent.CreateDynamicMaterialInstance` (`/Game/LianJiaCheng/Blueprint/Card/BP_DotIndicator.Decal` _returnvalue)))
                          (`MaterialInstanceDynamic.SetVectorParameterValue` _returnvalue_2 "BaseColor" (struct :`R` 1.0 :`A` 1.0))))))))))
          (:`then_1`
            ;;[1 1 1] Update Creeper Indicator Location
            (`/Engine/EditorBlueprintResources/StandardMacros.IsValid` _tmpchosencreeper
              (:`Is Valid`
                (`/Engine/EditorBlueprintResources/StandardMacros.IsValid` _tmpchosencreeperindicator_2
                  (:`Is Valid`
                    (`self.K2_SetActorLocation` _tmpchosencreeperindicator_2 (+ (`self.K2_GetActorLocation` _tmpchosencreeper) (`KismetMathLibrary.MakeVector` 0.0 0.0 20.0)) false false)))))))
        (else
          ;;[1 1 1] Clear Creeper Indicator
          (`/Engine/EditorBlueprintResources/StandardMacros.IsValid` _tmpchosencreeperindicator
            (:`Is Valid`
              (`self.K2_DestroyActor` _tmpchosencreeperindicator))))))))

(fn `CardEffectHandler`
  (params (CardEffectEnum :type "/Game/LianJiaCheng/Blueprint/Card/E_Card_Effect Enum" :default "NewEnumerator0") (CardUseEnum :type "/Game/LianJiaCheng/Blueprint/Card/E_Card_UseState Enum" :default "NewEnumerator0") (SlimeSide :type "/Game/LianJiaCheng/Blueprint/Slime/E_Slime_SideNum Enum" :default "NewEnumerator0"))
  (switch `/Game/LianJiaCheng/Blueprint/Card/E_Card_Effect` CardEffectEnum
    (:`NewEnumerator0`
      (`self.PrairieFire` CardUseEnum))
    (:`NewEnumerator1`
      (`self.NuwasHand` CardUseEnum))
    (:`NewEnumerator3`
      (`self.PowerfulWind` CardUseEnum))
    (:`NewEnumerator7`
      (`self.SlimesEvolution` CardUseEnum))
    (:`NewEnumerator4`
      (`self.SlimesRain` CardUseEnum SlimeSide))
    (:`NewEnumerator6`
      (`self.SlimeCreeper` CardUseEnum))))

(fn `GetMouseHit`
  (returns (HitActor :type "Actor Object Reference") (Location :type "Vector Structure"))
  (bind (_worldlocation _worlddirection) (`PlayerController.DeprojectMousePositionToWorld` (`GameplayStatics.GetPlayerController` 0)))
  (bind (_outhit _returnvalue) (`KismetSystemLibrary.LineTraceSingle` _worldlocation (+ _worldlocation (* _worlddirection 20000.0)) "TraceTypeQuery1"))
  (if _returnvalue
    (bind (_bblockinghit _binitialoverlap _time _distance _location _impactpoint _normal _impactnormal _physmat _hitactor) (`GameplayStatics.BreakHitResult` _outhit))
    (return _hitactor _location)))

(fn `NuwasHand`
  (params (UseState :type "/Game/LianJiaCheng/Blueprint/Card/E_Card_UseState Enum" :default "NewEnumerator0"))
  (bind _tmpindicator1 (`self.TmpIndicator1`))
  (bind _tmpindicator1_2 (`self.TmpIndicator1`))
  (bind _tmpindicator1_3 (`self.TmpIndicator1`))
  (switch `/Game/LianJiaCheng/Blueprint/Card/E_Card_UseState` UseState
    (:`NewEnumerator0`
      ;[1 1 1] Spawn Indicator
      (`/Engine/EditorBlueprintResources/StandardMacros.IsValid` _tmpindicator1_2
        (:`Is Valid`
          (`self.K2_DestroyActor` _tmpindicator1_2))
        (:`Is Not Valid`
          _))
      (bind _returnvalue (`|SpawnActorFromClass` "/Game/LianJiaCheng/Blueprint/Card/BP_DotIndicator.BP_DotIndicator_C" (`KismetMathLibrary.MakeTransform` (0.0 0.0 0.0)) "Undefined" "OverrideRootScale" null null))
      (`/Game/LianJiaCheng/Blueprint/Card/BP_DotIndicator.InitDecal` _returnvalue (`self.NuwasHandPreIndicatorRadius`) true)
      (set `self.TmpIndicator1` _returnvalue))
    (:`NewEnumerator1`
      ;[1 1 1] Spawn Range
      (`/Engine/EditorBlueprintResources/StandardMacros.IsValid` _tmpindicator1
        (:`Is Valid`
          (bind _returnvalue_2 (`|SpawnActorFromClass` "/Game/LianJiaCheng/Blueprint/Card/BP_GamePlayCue_NuwasHand.BP_GamePlayCue_NuwasHand_C" (`KismetMathLibrary.Conv_VectorToTransform` (`self.K2_GetActorLocation` _tmpindicator1)) "Undefined" "OverrideRootScale" null null))
          (`/Game/LianJiaCheng/Blueprint/Card/BP_GamePlayCue_NuwasHand.Start Nuwa` _returnvalue_2 (`self.NuwasHandPostIndicatorRadius`) (`self.NuwasHandEffectRadius`)))))
    (:`NewEnumerator7`
      ;[1 1 1] Cancel
      (`/Engine/EditorBlueprintResources/StandardMacros.IsValid` _tmpindicator1_3
        (:`Is Valid`
          (`self.K2_DestroyActor` _tmpindicator1_3))))))

(fn `PowerfulWind`
  (params (UseState :type "/Game/LianJiaCheng/Blueprint/Card/E_Card_UseState Enum" :default "NewEnumerator0"))
  (bind _tmpindicator1 (`self.TmpIndicator1`))
  (bind _tmpindicator1_2 (`self.TmpIndicator1`))
  (bind _tmpdecal1 (`self.TmpDecal1`))
  (bind _mildwindloopsound (`self.MildWindLoopSound`))
  (bind _tmpdecal1_2 (`self.TmpDecal1`))
  (bind _tmpdecal1_3 (`self.TmpDecal1`))
  (bind _tmpwinddecal2 (`self.TmpWindDecal2`))
  (bind _tmpwindstarteffect (`self.TmpWindStartEffect`))
  (switch `/Game/LianJiaCheng/Blueprint/Card/E_Card_UseState` UseState
    (:`NewEnumerator0`
      ;[1 1 1] Spawn Indicator
      ;;[1 1 1] Clear ld
      (`/Engine/EditorBlueprintResources/StandardMacros.IsValid` _tmpindicator1
        (:`Is Valid`
          (`self.K2_DestroyActor` _tmpindicator1))
        (:`Is Not Valid`
          _))
      (bind _returnvalue (`|SpawnActorFromClass` "/Game/LianJiaCheng/Blueprint/Card/BP_RangeIndicator.BP_RangeIndicator_C" (`KismetMathLibrary.MakeTransform` (0.0 0.0 0.0)) "Undefined" "OverrideRootScale" null null))
      (`/Game/LianJiaCheng/Blueprint/Card/BP_RangeIndicator.InitDecal` _returnvalue (`self.WindTornadoRadius`))
      (set `self.TmpIndicator1` _returnvalue))
    (:`NewEnumerator1`
      (`/Engine/EditorBlueprintResources/StandardMacros.IsValid` (`self.TmpIndicator1`)
        (:`Is Valid`
          (`|ExecutionSequence`
            (:`then_0`
              ;[1 1 1] Spawn Decal1
              (bind _returnvalue_2 (`GameplayStatics.SpawnDecalAtLocation` "/Game/LianJiaCheng/Material/M_RangeTarget.M_RangeTarget" (`KismetMathLibrary.Conv_DoubleToVector` (`self.WindTornadoRadius`)) (`self.K2_GetActorLocation` (`self.TmpIndicator1`))))
              (set `self.TmpDecal1` _returnvalue_2)
              ;[1 1 1] Clear Indicator
              (`self.K2_DestroyActor` (`self.TmpIndicator1`)))
            (:`then_1`
              ;[1 1 1] Spawn Tmp Effect
              (bind _returnvalue_3 (`NiagaraFunctionLibrary.SpawnSystemAtLocation` "/Game/LianJiaCheng/Effect/VFX_Wind_Pack/VFX_Niagara/NS_Wind_Whirlwind.NS_Wind_Whirlwind" (`SceneComponent.K2_GetComponentLocation` _tmpdecal1_3) (struct) (`KismetMathLibrary.Conv_DoubleToVector` (/ (.y (`DecalComponent.DecalSize` _tmpdecal1_3)) (`self.WindWhirlwindOriginalRadius`)))))
              (set `self.TmpWindStartEffect` _returnvalue_3))
            (:`then_2`
              ;[1 1 1] Play WindBegin Sound
              (bind _returnvalue_4 (`GameplayStatics.SpawnSound2D` "/Game/LianJiaCheng/Sound/S_MildWindLoop.S_MildWindLoop" 1.0 1.0 0.0 null false false))
              (bind _output_get (set `self.MildWindLoopSound` _returnvalue_4))
              (`AudioComponent.Play` _output_get 0.0))
            (:`then_3`
              ;[1 1 1] Play Camera Shake
              (`GameplayStatics.PlayWorldCameraShake` "/Game/LianJiaCheng/Effect/BP_CameraShake_WindStart.BP_CameraShake_WindStart_C" (`self.K2_GetActorLocation` (`GameplayStatics.GetPlayerCameraManager` 0)) 10.0 100.0))
            (:`then_4`
              ;[1 1 1] Spawn Decal2
              (set `self.IsWinding` true)
              (bind _returnvalue_5 (`GameplayStatics.SpawnDecalAtLocation` "/Game/LianJiaCheng/Material/M_Arrow.M_Arrow" (`KismetMathLibrary.Conv_DoubleToVector` (`self.WindArrowIndicatorRadius`)) (`SceneComponent.K2_GetComponentLocation` (`self.TmpDecal1`))))
              (set `self.TmpWindDecal2` _returnvalue_5))
            (:`then_5`
              ;[1 1 1] DarkPPV
              (`self.SkyDarken`))))))
    (:`NewEnumerator3`
      ;[1 1 1] Spawn Dir
      (set `self.IsWinding` false)
      (`/Engine/EditorBlueprintResources/StandardMacros.IsValid` _tmpdecal1
        (:`Is Valid`
          (bind _returnvalue_6 (`|SpawnActorFromClass` "/Game/LianJiaCheng/Blueprint/Card/BP_GaemPlayCue_PowerfulWind.BP_GaemPlayCue_PowerfulWind_C" (`KismetMathLibrary.Conv_VectorToTransform` (`SceneComponent.K2_GetComponentLocation` _tmpdecal1)) "Undefined" "OverrideRootScale" null null))
          (`|ExecutionSequence`
            (:`then_0`
              ;[1 1 1] Stop Camera Shake
              (`PlayerCameraManager.StopAllCameraShakes` (`GameplayStatics.GetPlayerCameraManager` 0) true))
            (:`then_1`
              ;[1 1 1] StartEffect
              (`/Game/LianJiaCheng/Blueprint/Card/BP_GaemPlayCue_PowerfulWind.StartWind` _returnvalue_6 (`SceneComponent.K2_GetComponentLocation` (`self.TmpDecal1`)) (`SceneComponent.K2_GetComponentLocation` (`self.TmpWindDecal2`)) (`self.WindTornadoRadius`)))))))
    (:`NewEnumerator2`
      (`|ExecutionSequence`
        (:`then_0`
          ;[1 1 1] PPV
          (`self.SkyLighten`))
        (:`then_1`
          ;[1 1 1] Cancel1
          (set `self.IsWinding` false :!label _label)
          (`/Engine/EditorBlueprintResources/StandardMacros.IsValid` _tmpindicator1_2
            (:`Is Valid`
              (`self.K2_DestroyActor` _tmpindicator1_2))
            (:`Is Not Valid`
              _))
          (`/Engine/EditorBlueprintResources/StandardMacros.IsValid` _tmpdecal1_2
            (:`Is Valid`
              (`ActorComponent.K2_DestroyComponent` _tmpdecal1_2))
            (:`Is Not Valid`
              _))
          (`/Engine/EditorBlueprintResources/StandardMacros.IsValid` _tmpwindstarteffect
            (:`Is Valid`
              (`ActorComponent.K2_DestroyComponent` _tmpwindstarteffect))
            (:`Is Not Valid`
              _))
          (`/Engine/EditorBlueprintResources/StandardMacros.IsValid` _tmpwinddecal2
            (:`Is Valid`
              (`ActorComponent.K2_DestroyComponent` _tmpwinddecal2))
            (:`Is Not Valid`
              _))
          (`/Engine/EditorBlueprintResources/StandardMacros.IsValid` _mildwindloopsound
            (:`Is Valid`
              (`ActorComponent.K2_DestroyComponent` _mildwindloopsound))))))
    (:`NewEnumerator7`
      (goto _label))))

(fn `PrairieFire`
  (params (UseState :type "/Game/LianJiaCheng/Blueprint/Card/E_Card_UseState Enum" :default "NewEnumerator0"))
  (bind _tmpindicator1 (`self.TmpIndicator1`))
  (bind _tmpindicator1_2 (`self.TmpIndicator1`))
  (bind _tmpindicator1_3 (`self.TmpIndicator1`))
  (switch `/Game/LianJiaCheng/Blueprint/Card/E_Card_UseState` UseState
    (:`NewEnumerator0`
      ;[1 1 1] Spawn Indicator
      (`/Engine/EditorBlueprintResources/StandardMacros.IsValid` _tmpindicator1_2
        (:`Is Valid`
          (`self.K2_DestroyActor` _tmpindicator1_2))
        (:`Is Not Valid`
          _))
      (bind _returnvalue (`|SpawnActorFromClass` "/Game/LianJiaCheng/Blueprint/Card/BP_RangeIndicator.BP_RangeIndicator_C" (`KismetMathLibrary.MakeTransform` (0.0 0.0 0.0)) "Undefined" "OverrideRootScale" null null))
      (`/Game/LianJiaCheng/Blueprint/Card/BP_RangeIndicator.InitDecal` _returnvalue (`self.PrairieFireEffectRadius`))
      (set `self.TmpIndicator1` _returnvalue))
    (:`NewEnumerator1`
      (`|ExecutionSequence`
        (:`then_0`
          ;[1 1 1] Spawn GamePlayCue
          (`/Engine/EditorBlueprintResources/StandardMacros.IsValid` _tmpindicator1
            (:`Is Valid`
              (bind _returnvalue_2 (`|SpawnActorFromClass` "/Game/LianJiaCheng/Blueprint/Card/BP_GamePlayCue_PrairieFire.BP_GamePlayCue_PrairieFire_C" (`KismetMathLibrary.Conv_VectorToTransform` (`self.K2_GetActorLocation` _tmpindicator1)) "Undefined" "OverrideRootScale" null null))
              (`/Game/LianJiaCheng/Blueprint/Card/BP_GamePlayCue_PrairieFire.StartFire` _returnvalue_2 (`self.PrairieFireEffectRadius`) (`self.ExplosionEffectRadius`)))))
        (:`then_1`
          ;[1 1 1] PPV
          (`self.SkyDarken`))))
    (:`NewEnumerator7`
      ;[1 1 1] Cancel
      (`/Engine/EditorBlueprintResources/StandardMacros.IsValid` _tmpindicator1_3
        (:`Is Valid`
          (`self.K2_DestroyActor` _tmpindicator1_3))))))

(fn `SlimeCreeper`
  (params (UseState :type "/Game/LianJiaCheng/Blueprint/Card/E_Card_UseState Enum" :default "NewEnumerator0"))
  (bind _tmpindicator1 (`self.TmpIndicator1`))
  (bind _tmpindicator1_2 (`self.TmpIndicator1`))
  (bind _tmpindicator1_3 (`self.TmpIndicator1`))
  (switch `/Game/LianJiaCheng/Blueprint/Card/E_Card_UseState` UseState
    (:`NewEnumerator0`
      ;[1 1 1] Spawn Indicator
      (set `self.IsChoosingCreeper` true)
      (`/Engine/EditorBlueprintResources/StandardMacros.IsValid` _tmpindicator1_2
        (:`Is Valid`
          (`self.K2_DestroyActor` _tmpindicator1_2))
        (:`Is Not Valid`
          _))
      (bind _returnvalue (`|SpawnActorFromClass` "/Game/LianJiaCheng/Blueprint/Card/BP_DotIndicator.BP_DotIndicator_C" (`KismetMathLibrary.MakeTransform` (0.0 0.0 0.0)) "Undefined" "OverrideRootScale" null null))
      (`/Game/LianJiaCheng/Blueprint/Card/BP_DotIndicator.InitDecal` _returnvalue (`self.NuwasHandPreIndicatorRadius`) true)
      (set `self.TmpIndicator1` _returnvalue))
    (:`NewEnumerator1`
      ;[1 1 1] Confirm Creeper
      (`/Engine/EditorBlueprintResources/StandardMacros.IsValid` _tmpindicator1
        (:`Is Valid`
          (bind _returnvalue_2 (`|SpawnActorFromClass` "/Game/LianJiaCheng/Blueprint/Card/BP_GamePlayCue_SlimeCreeper.BP_GamePlayCue_SlimeCreeper_C" (`KismetMathLibrary.Conv_VectorToTransform` (`self.K2_GetActorLocation` _tmpindicator1)) "Undefined" "OverrideRootScale" null null))
          (`/Game/LianJiaCheng/Blueprint/Card/BP_GamePlayCue_SlimeCreeper.StartCreeper` _returnvalue_2 (`self.TmpChosenCreeper`) (`self.CreeperExplosionRadius`)))))
    (:`NewEnumerator7`
      ;[1 1 1] Cancel
      (set `self.IsChoosingCreeper` false)
      (`/Engine/EditorBlueprintResources/StandardMacros.IsValid` _tmpindicator1_3
        (:`Is Valid`
          (`self.K2_DestroyActor` _tmpindicator1_3))))))

(fn `SlimesEvolution`
  (params (UseState :type "/Game/LianJiaCheng/Blueprint/Card/E_Card_UseState Enum" :default "NewEnumerator0"))
  (bind _tmpindicator1 (`self.TmpIndicator1`))
  (bind _tmpindicator1_2 (`self.TmpIndicator1`))
  (bind _tmpindicator1_3 (`self.TmpIndicator1`))
  (switch `/Game/LianJiaCheng/Blueprint/Card/E_Card_UseState` UseState
    (:`NewEnumerator0`
      ;[1 1 1] Spawn Indicator
      (`/Engine/EditorBlueprintResources/StandardMacros.IsValid` _tmpindicator1_2
        (:`Is Valid`
          (`self.K2_DestroyActor` _tmpindicator1_2))
        (:`Is Not Valid`
          _))
      (bind _returnvalue (`|SpawnActorFromClass` "/Game/LianJiaCheng/Blueprint/Card/BP_RangeIndicator.BP_RangeIndicator_C" (`KismetMathLibrary.MakeTransform` (0.0 0.0 0.0)) "Undefined" "OverrideRootScale" null null))
      (`/Game/LianJiaCheng/Blueprint/Card/BP_RangeIndicator.InitDecal` _returnvalue (`self.EvolutionEffectRadius`))
      (set `self.TmpIndicator1` _returnvalue))
    (:`NewEnumerator1`
      (`|ExecutionSequence`
        (:`then_0`
          ;[1 1 1] Spawn Range
          (`/Engine/EditorBlueprintResources/StandardMacros.IsValid` _tmpindicator1
            (:`Is Valid`
              (bind _returnvalue_2 (`|SpawnActorFromClass` "/Game/LianJiaCheng/Blueprint/Card/BP_GamePlayCue_SlimesEvolution.BP_GamePlayCue_SlimesEvolution_C" (`KismetMathLibrary.Conv_VectorToTransform` (+ (`self.K2_GetActorLocation` _tmpindicator1) (`KismetMathLibrary.MakeVector` 0.0 0.0 20.0))) "Undefined" "OverrideRootScale" null null))
              (`/Game/LianJiaCheng/Blueprint/Card/BP_GamePlayCue_SlimesEvolution.StartEvolution` _returnvalue_2 (`self.EvolutionEffectRadius`)))))
        (:`then_1`
          ;[1 1 1] PPV
          (`self.SkyDarken`))))
    (:`NewEnumerator7`
      ;[1 1 1] Cancel
      (`/Engine/EditorBlueprintResources/StandardMacros.IsValid` _tmpindicator1_3
        (:`Is Valid`
          (`self.K2_DestroyActor` _tmpindicator1_3))))))

(fn `SlimesRain`
  (params (UseState :type "/Game/LianJiaCheng/Blueprint/Card/E_Card_UseState Enum" :default "NewEnumerator0") (SlimeSide :type "/Game/LianJiaCheng/Blueprint/Slime/E_Slime_SideNum Enum" :default "NewEnumerator0"))
  (bind _tmpindicator1 (`self.TmpIndicator1`))
  (bind _tmpindicator1_2 (`self.TmpIndicator1`))
  (bind _tmpindicator1_3 (`self.TmpIndicator1`))
  (switch `/Game/LianJiaCheng/Blueprint/Card/E_Card_UseState` UseState
    (:`NewEnumerator0`
      ;[1 1 1] Spawn Indicator
      (`/Engine/EditorBlueprintResources/StandardMacros.IsValid` _tmpindicator1_2
        (:`Is Valid`
          (`self.K2_DestroyActor` _tmpindicator1_2))
        (:`Is Not Valid`
          _))
      (bind _returnvalue (`|SpawnActorFromClass` "/Game/LianJiaCheng/Blueprint/Card/BP_RangeIndicator.BP_RangeIndicator_C" (`KismetMathLibrary.MakeTransform` (0.0 0.0 0.0)) "Undefined" "OverrideRootScale" null null))
      (`/Game/LianJiaCheng/Blueprint/Card/BP_RangeIndicator.InitDecal` _returnvalue (`self.RainEffectRadius`))
      (set `self.TmpIndicator1` _returnvalue))
    (:`NewEnumerator1`
      ;[1 1 1] Spawn Range
      (`/Engine/EditorBlueprintResources/StandardMacros.IsValid` _tmpindicator1
        (:`Is Valid`
          (bind _returnvalue_2 (`|SpawnActorFromClass` "/Game/LianJiaCheng/Blueprint/Card/BP_GamePlayCue_SlimesRain.BP_GamePlayCue_SlimesRain_C" (`KismetMathLibrary.Conv_VectorToTransform` (`self.K2_GetActorLocation` _tmpindicator1)) "Undefined" "OverrideRootScale" null null))
          (`/Game/LianJiaCheng/Blueprint/Card/BP_GamePlayCue_SlimesRain.StartRain` _returnvalue_2 SlimeSide (`self.RainEffectRadius`)))))
    (:`NewEnumerator7`
      ;[1 1 1] Cancel
      (`/Engine/EditorBlueprintResources/StandardMacros.IsValid` _tmpindicator1_3
        (:`Is Valid`
          (`self.K2_DestroyActor` _tmpindicator1_3))))))

(fn `UserConstructionScript`)