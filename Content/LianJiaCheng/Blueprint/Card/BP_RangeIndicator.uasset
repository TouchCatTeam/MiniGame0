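; Range indicator actor that follows the mouse cursor in the world, showing an area of a given radius.
; InitDecal scales the decal and the sphere to that radius and makes the sphere visible in game.
; Each tick, GetMouseHit traces the Visibility channel from the deprojected cursor and moves the actor to the hit location.
; A ray-plane intersection helper, GetMousePosition, is also defined but not called here.
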(event `InitDecal`
  (params (DecalRadius :type "Float (double-precision)" :default 128.0))
  (bind _sphere (`self.Sphere`))
  ;[1 1 1] Spawn Decal
  (`SceneComponent.SetWorldScale3D` (`self.Decal`) (`KismetMathLibrary.Conv_DoubleToVector` (/ DecalRadius (`self.TargetDecalOriginalRadius`))))
  ;[1 1 1] Init Sphere
  (`SceneComponent.SetWorldScale3D` _sphere (`KismetMathLibrary.Conv_DoubleToVector` (/ DecalRadius 50.0)))
  (`SceneComponent.SetHiddenInGame` _sphere false false))

(event `self.ReceiveTick`
  (params (DeltaSeconds :type "Float (single-precision)"))
  ;[1 1 1] Update Location
  (bind (_hitactor _location) (`self.GetMouseHit`))
  (`self.K2_SetActorLocation` _location))

(fn `GetMouseHit`
  (returns (HitActor :type "Actor Object Reference") (Location :type "Vector Structure"))
  (bind (_worldlocation _worlddirection) (`PlayerController.DeprojectMousePositionToWorld` (`GameplayStatics.GetPlayerController` 0)))
  (bind (_outhit _returnvalue) (`KismetSystemLibrary.LineTraceSingle` _worldlocation (+ _worldlocation (* _worlddirection 20000.0)) "TraceTypeQuery1"))
  (if _returnvalue
    (bind (_bblockinghit _binitialoverlap _time _distance _location _impactpoint _normal _impactnormal _physmat _hitactor) (`GameplayStatics.BreakHitResult` _outhit))
    (return _hitactor _location)))

(fn `GetMousePosition`
  (params (NewParam :type "Vector Structure") (NewParam1 :type "Rotator Structure"))
  (returns (NewParam :type "Vector Structure"))
  (locals (n :type "Vector Structure") (d :type "Float (double-precision)") (t :type "Float (double-precision)"))
  (bind _n (`local.n`))
  (bind (_worldlocation _worlddirection) (`PlayerController.DeprojectMousePositionToWorld` (`GameplayStatics.GetPlayerController` 0)))
  (set `local.n` (`KismetMathLibrary.GetUpVector` NewParam1))
  (set `local.d` (`KismetMathLibrary.Dot_VectorVector` NewParam (`local.n`)))
  (set `local.t` (/ (- (`local.d`) (`KismetMathLibrary.Dot_VectorVector` _worldlocation _n)) (`KismetMathLibrary.Dot_VectorVector` _n _worlddirection)))
  (return (+ _worldlocation (* _worlddirection (`local.t`)))))

(fn `UserConstructionScript`)