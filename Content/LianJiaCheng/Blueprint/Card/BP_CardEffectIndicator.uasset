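; Card effect targeting indicator actor that follows the mouse cursor and tracks which slimes sit inside its area.
; While ShouldUpdatePos is set, Tick moves it to a visibility trace hit under the cursor and runs a projectile path prediction whose result is unused.
; Sphere overlap events add and remove BP_Slime_Parent actors in SlimesInRange.
; A ray-plane intersection helper, GetMousePosition, is defined but not called here.
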(event `self.ReceiveTick`
  (params (DeltaSeconds :type "Float (single-precision)"))
  (bind _returnvalue (`self.K2_GetActorLocation` self))
  (if (`self.ShouldUpdatePos`)
    ;[1 1 1] Update Location
    (bind (_hitactor _location) (`self.GetMouseHit`))
    (`self.K2_SetActorLocation` _location)
    (`GameplayStatics.Blueprint_PredictProjectilePath_ByObjectType` _returnvalue (* (`KismetMathLibrary.MakeVector` (.x (`KismetMathLibrary.GetDirectionUnitVector` _returnvalue _location)) (.y (`KismetMathLibrary.GetDirectionUnitVector` _returnvalue _location)) (+ (.z (`KismetMathLibrary.GetDirectionUnitVector` _returnvalue _location)) 0.25)) 2000.0) true 0.0 (`|MakeArray` "ObjectTypeQuery1" :!type "EObjectTypeQuery Enum"))))

(event `self.Sphere.OnComponentBeginOverlap`
  (params (OverlappedComponent :type "PrimitiveComponent Object Reference") (OtherActor :type "Actor Object Reference") (OtherComp :type "PrimitiveComponent Object Reference") (OtherBodyIndex :type Integer) (bFromSweep :type Boolean) (SweepResult :type "HitResult Structure (by ref)"))
  ;[1 1 1] Get Slimes In Range
  (bind _asbp_slime_parent (cast `/Game/LianJiaCheng/Blueprint/Slime/BP_Slime_Parent` OtherActor))
  (`KismetArrayLibrary.Array_Add` (`self.SlimesInRange`) _asbp_slime_parent))

(event `self.Sphere.OnComponentEndOverlap`
  (params (OverlappedComponent :type "PrimitiveComponent Object Reference") (OtherActor :type "Actor Object Reference") (OtherComp :type "PrimitiveComponent Object Reference") (OtherBodyIndex :type Integer))
  ;[1 1 1] Get Slimes In Range
  (bind _asbp_slime_parent (cast `/Game/LianJiaCheng/Blueprint/Slime/BP_Slime_Parent` OtherActor))
  (`KismetArrayLibrary.Array_RemoveItem` (`self.SlimesInRange`) _asbp_slime_parent))

(fn `GetMouseHit`
  (returns (HitActor :type "Actor Object Reference") (Location :type "Vector Structure"))
  (bind (_worldlocation _worlddirection) (`PlayerController.DeprojectMousePositionToWorld` (`GameplayStatics.GetPlayerController` 0)))
  (bind (_outhit _returnvalue) (`KismetSystemLibrary.LineTraceSingle` _worldlocation (+ _worldlocation (* _worlddirection 20000.0)) "TraceTypeQuery1"))
  (if _returnvalue
    (bind (_bblockinghit _binitialoverlap _time _distance _location _impactpoint _normal _impactnormal _physmat _hitactor) (`GameplayStatics.BreakHitResult` _outhit))
    (return _hitactor _location)))

(fn `GetMousePosition`
  (params (NewParam :type "Vector Structure") (NewParam1 :type "Rotator Structure"))
  (returns (NewParam :type "Vector Structure"))
  (locals (n :type "Vector Structure") (d :type "Float (double-precision)") (t :type "Float (double-precision)"))
  (bind _n (`local.n`))
  (bind (_worldlocation _worlddirection) (`PlayerController.DeprojectMousePositionToWorld` (`GameplayStatics.GetPlayerController` 0)))
  (set `local.n` (`KismetMathLibrary.GetUpVector` NewParam1))
  (set `local.d` (`KismetMathLibrary.Dot_VectorVector` NewParam (`local.n`)))
  (set `local.t` (/ (- (`local.d`) (`KismetMathLibrary.Dot_VectorVector` _worldlocation _n)) (`KismetMathLibrary.Dot_VectorVector` _n _worlddirection)))
  (return (+ _worldlocation (* _worlddirection (`local.t`)))))

(fn `UserConstructionScript`)