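; Card effect actor that makes slimes rain down around its location for a given side, then destroys itself.
; StartRain spawns a radius-scaled particle effect overhead, waits briefly, spawns a batch of slimes at that height, then cleans up after another delay.
; SpawnNewSlime scatters positions with square-root radius sampling, assigns side and random class, and launches each slime within a downward cone.
; A mouse-trace helper, GetMouseHit, is defined but not called here.
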(event `StartRain`
  (params (SideNum :type "/Game/LianJiaCheng/Blueprint/Slime/E_Slime_SideNum Enum" :default "NewEnumerator0") (RainRadius :type "Float (double-precision)" :default 900.0))
  (bind _returnvalue (+ (`self.K2_GetActorLocation` self) (`KismetMathLibrary.MakeVector` 0.0 0.0 800.0)))
  (`|ExecutionSequence`
    (:`then_0`
      ;[1 1 1] Init
      (set `self.SideNum` SideNum))
    (:`then_1`
      ;[1 1 1] Spawn Effect
      (bind _returnvalue_2 (`GameplayStatics.SpawnEmitterAtLocation` "/Game/LianJiaCheng/Effect/MagicCircles2/ParticleSystems/PS_SlimesRain.PS_SlimesRain" _returnvalue (struct :`Roll` 180.0) (`KismetMathLibrary.Conv_DoubleToVector` (/ RainRadius (`self.RainEffectOriginalRadius`)))))
      (set `self.PSToPlay` _returnvalue_2))
    (:`then_2`
      ;[1 1 1] Spawn Slime
      (`KismetSystemLibrary.Delay` 1.0)
      (for _ (range 10)
        (`self.SpawnNewSlime` _returnvalue (`self.SideNum`) RainRadius))
      (`KismetSystemLibrary.Delay` 1.0)
      ;[1 1 1] End
      (`ActorComponent.K2_DestroyComponent` (`self.PSToPlay`))
      (`self.K2_DestroyActor`))))

(fn `GetMouseHit`
  (returns (MouseHitPos :type "Vector Structure") (IsHit :type Boolean))
  (bind (_worldlocation _worlddirection) (`PlayerController.DeprojectMousePositionToWorld` (`GameplayStatics.GetPlayerController` 0)))
  (bind (_outhit _returnvalue) (`KismetSystemLibrary.LineTraceSingle` _worldlocation (+ _worldlocation (* _worlddirection 20000.0)) "TraceTypeQuery1"))
  (if _returnvalue
    (return (`.Location` (`GameplayStatics.BreakHitResult` _outhit)) true)
    (else
      (return (0.0 0.0 0.0) false))))

(fn `SpawnNewSlime`
  (params (SpawnPos :type "Vector Structure") (SideNum :type "/Game/LianJiaCheng/Blueprint/Slime/E_Slime_SideNum Enum" :default "NewEnumerator0") (RainRadius :type "Float (double-precision)"))
  (bind _returnvalue (`KismetMathLibrary.RandomFloatInRange` 0.0 360.0))
  (bind _returnvalue_2 (* RainRadius (`KismetMathLibrary.Sqrt` (`KismetMathLibrary.RandomFloatInRange` 0.0 1.0))))
  (bind _returnvalue_3 (`|SpawnActorFromClass` "/Game/LianJiaCheng/Blueprint/Slime/BP_Slime_Parent.BP_Slime_Parent_C" (`KismetMathLibrary.Conv_VectorToTransform` (`KismetMathLibrary.MakeVector` (+ (.x SpawnPos) (* _returnvalue_2 (`KismetMathLibrary.DegCos` _returnvalue))) (+ (.y SpawnPos) (* _returnvalue_2 (`KismetMathLibrary.DegSin` _returnvalue))) (.z SpawnPos))) "Undefined" "OverrideRootScale" null null))
  (`/Engine/EditorBlueprintResources/StandardMacros.IsValid` _returnvalue_3
    (:`Is Valid`
      (set `/Game/LianJiaCheng/Blueprint/Slime/BP_Slime_Parent.SideEnum` SideNum _returnvalue_3)
      (switch `int` (`KismetMathLibrary.RandomIntegerInRange` 0 3)
        (:`0`
          (set `/Game/LianJiaCheng/Blueprint/Slime/BP_Slime_Parent.ClassEnum` "NewEnumerator0" _returnvalue_3))
        (:`1`
          (set `/Game/LianJiaCheng/Blueprint/Slime/BP_Slime_Parent.ClassEnum` "NewEnumerator1" _returnvalue_3))
        (:`2`
          (set `/Game/LianJiaCheng/Blueprint/Slime/BP_Slime_Parent.ClassEnum` "NewEnumerator2" _returnvalue_3))
        (:`3`
          (set `/Game/LianJiaCheng/Blueprint/Slime/BP_Slime_Parent.ClassEnum` "NewEnumerator3" _returnvalue_3)))
      (`/Game/LianJiaCheng/Blueprint/Slime/BP_Slime_Parent.RefreshSlimeComponent` _returnvalue_3)
      (`Character.LaunchCharacter` _returnvalue_3 (* (`KismetMathLibrary.RandomUnitVectorInConeInDegrees` (0.0 0.0 -1.0) 60.0) 300.0) false false))))

(fn `UserConstructionScript`)