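; Gameplay cue actor for a slime evolution card that upgrades male and female slimes within a radius to their Pro classes.
; StartEvolution spawns a scaled shield effect with sound, then resizes an overlap sphere, whose begin/end events maintain the in-range slime list.
; Each listed slime of an eligible class switches its class enum, refreshes its components and plays a level-up sound.
; After a delay, it calls SkyLighten on BP_CardRepertory and destroys itself and the effect.
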(event `StartEvolution`
  (params (EvolutionEffectRadius :type "Float (double-precision)" :default 650.0))
  (`|ExecutionSequence`
    (:`then_0`
      ;[1 1 1] Spawn Effect
      (bind _returnvalue (`GameplayStatics.SpawnEmitterAtLocation` "/Game/LianJiaCheng/Effect/MagicCircles2/ParticleSystems/PS_NanoShield.PS_NanoShield" (+ (`self.K2_GetActorLocation`) (`KismetMathLibrary.MakeVector` 0.0 0.0 10.0)) (struct) (`KismetMathLibrary.Conv_DoubleToVector` (/ EvolutionEffectRadius (`self.EvolutionEffectOriginalRadius`)))))
      (set `self.EffectToPlay` _returnvalue)
      ;[1 1 1] Play MagicCircle Sound
      (`GameplayStatics.PlaySound2D` "/Game/LianJiaCheng/Sound/SCue_MagicCircle.SCue_MagicCircle" 1.0 1.0 0.0 null null))
    (:`then_1`
      ;[1 1 1] Init Sphere
      (`SphereComponent.SetSphereRadius` (`self.Sphere`) EvolutionEffectRadius true))
    (:`then_2`
      ;[1 1 1] Slime in Range Evolute
      (for _array_element (`self.SlimesInRange`)
        (`self.Evolute` _array_element)))
    (:`then_3`
      ;[1 1 1] End
      (`KismetSystemLibrary.Delay` 4.0)
      (`|ExecutionSequence`
        (:`then_0`
          ;[1 1 1] PPV
          (bind _returnvalue_2 (`GameplayStatics.GetActorOfClass` "/Game/LianJiaCheng/Blueprint/Card/BP_CardRepertory.BP_CardRepertory_C"))
          (`/Game/LianJiaCheng/Blueprint/Card/BP_CardRepertory.SkyLighten` _returnvalue_2))
        (:`then_1`
          ;[1 1 1] Destroy
          (`ActorComponent.K2_DestroyComponent` (`self.EffectToPlay`))
          (`self.K2_DestroyActor`))))))

(event `self.Sphere.OnComponentBeginOverlap`
  (params (OverlappedComponent :type "PrimitiveComponent Object Reference") (OtherActor :type "Actor Object Reference") (OtherComp :type "PrimitiveComponent Object Reference") (OtherBodyIndex :type Integer) (bFromSweep :type Boolean) (SweepResult :type "HitResult Structure (by ref)"))
  ;[1 1 1] Get Slimes In Range
  (bind _asbp_slime_parent (cast `/Game/LianJiaCheng/Blueprint/Slime/BP_Slime_Parent` OtherActor))
  (`KismetArrayLibrary.Array_Add` (`self.SlimesInRange`) _asbp_slime_parent))

(event `self.Sphere.OnComponentEndOverlap`
  (params (OverlappedComponent :type "PrimitiveComponent Object Reference") (OtherActor :type "Actor Object Reference") (OtherComp :type "PrimitiveComponent Object Reference") (OtherBodyIndex :type Integer))
  ;[1 1 1] Get Slimes In Range
  (bind _asbp_slime_parent (cast `/Game/LianJiaCheng/Blueprint/Slime/BP_Slime_Parent` OtherActor))
  (`KismetArrayLibrary.Array_RemoveItem` (`self.SlimesInRange`) _asbp_slime_parent))

(fn `Evolute`
  (params (Actor :type "Actor Object Reference"))
  (bind _asbp_slime_parent (cast `/Game/LianJiaCheng/Blueprint/Slime/BP_Slime_Parent` Actor))
  (switch `/Game/LianJiaCheng/Blueprint/Slime/E_Slime_ClassNum` (`/Game/LianJiaCheng/Blueprint/Slime/BP_Slime_Parent.ClassEnum` _asbp_slime_parent)
    (:`NewEnumerator0`
      (set `/Game/LianJiaCheng/Blueprint/Slime/BP_Slime_Parent.ClassEnum` "NewEnumerator1" _asbp_slime_parent)
      (`/Game/LianJiaCheng/Blueprint/Slime/BP_Slime_Parent.RefreshSlimeComponent` _asbp_slime_parent)
      (`GameplayStatics.PlaySound2D` "/Game/LianJiaCheng/Sound/SCue_LevelUp.SCue_LevelUp" 1.0 1.0 0.0 null null))
    (:`NewEnumerator2`
      (set `/Game/LianJiaCheng/Blueprint/Slime/BP_Slime_Parent.ClassEnum` "NewEnumerator3" _asbp_slime_parent)
      (`/Game/LianJiaCheng/Blueprint/Slime/BP_Slime_Parent.RefreshSlimeComponent` _asbp_slime_parent)
      (`GameplayStatics.PlaySound2D` "/Game/LianJiaCheng/Sound/SCue_LevelUp.SCue_LevelUp" 1.0 1.0 0.0 null null))))

(fn `UserConstructionScript`)