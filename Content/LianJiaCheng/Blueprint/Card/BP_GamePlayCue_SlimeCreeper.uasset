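; Gameplay cue actor for the Creeper slime card, turning a slime into a creeper that explodes when destroyed.
; StartCreeper swaps in the active material, plays a match sound, stores the radius and judger, and binds to the slime's OnDestroyed.
; The explosion plays scaled effects, shake and sound, then launches every judger-listed slime.
; Slimes within radius of the cue actor fly randomly and die a second later, when the cue destroys itself.
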(event `StartCreeper`
  (params (CreeperActor :type "Actor Object Reference") (CreeperExplosionRadius :type "Float (double-precision)" :default 900.0))
  (bind _asbp_slime_parent (cast `/Game/LianJiaCheng/Blueprint/Slime/BP_Slime_Parent` CreeperActor))
  (`|ExecutionSequence`
    (:`then_0`
      ;[1 1 1] Set Creeper Slime
      (`PrimitiveComponent.SetMaterial` (`Character.Mesh` _asbp_slime_parent) 0 (`/Game/LianJiaCheng/Blueprint/Slime/BP_Slime_Parent.CreeperActiveMaterial` _asbp_slime_parent))
      (add `self.OnDestroyed` _asbp_slime_parent (`|CreateDelegate` :!event `Creeper Explose`)))
    (:`then_1`
      ;[1 1 1] Init Radius
      (set `self.CreeperExplosionEffectRadius` CreeperExplosionRadius))
    (:`then_2`
      ;[1 1 1] Get Judger
      (bind _outactors (`GameplayStatics.GetAllActorsOfClass` "/Game/LianJiaCheng/Blueprint/Judger/BP_Judger.BP_Judger_C"))
      (set `self.Judger` (`|GetArrayItem` _outactors)))
    (:`then_3`
      ;[1 1 1] Play Creeper Active Sound
      (`GameplayStatics.PlaySound2D` "/Game/LianJiaCheng/Sound/S_StrikeMatch.S_StrikeMatch" 1.0 1.0 0.0 null null))))

(event `Creeper Explose` :!signature `self.OnDestroyed`
  (params (DestroyedActor :type "Actor Object Reference"))
  (`|ExecutionSequence`
    (:`then_0`
      ;[1 1 1] Spawn Explosion Effect
      (bind _returnvalue (`NiagaraFunctionLibrary.SpawnSystemAtLocation` "/Game/LianJiaCheng/Effect/Explosions_Niagara/Particles/P_Explosion03.P_Explosion03" (`self.K2_GetActorLocation` DestroyedActor) (struct) (`KismetMathLibrary.Conv_DoubleToVector` (/ (`self.CreeperExplosionEffectRadius`) (`self.CreeperExplosionEffectOriginalRadius`)))))
      (set `self.CreeperExplosionToPlay` _returnvalue)
      ;[1 1 1] Wait for Effect Complete
      (`KismetSystemLibrary.Delay` 2.0)
      (`ActorComponent.K2_DestroyComponent` (`self.CreeperExplosionToPlay`)))
    (:`then_1`
      ;[1 1 1] Play Camera Shake
      (`GameplayStatics.PlayWorldCameraShake` "/Game/LianJiaCheng/Effect/BP_CameraSkake_Explosion.BP_CameraSkake_Explosion_C" (`self.K2_GetActorLocation` (`GameplayStatics.GetPlayerCameraManager` 0)) 10.0 100.0))
    (:`then_2`
      ;[1 1 1] Play CreeperExplosion Sound
      (`GameplayStatics.PlaySound2D` "/Game/LianJiaCheng/Sound/SCue_Explosion.SCue_Explosion" 1.0 1.0 0.0 null null))
    (:`then_3`
      ;[1 1 1] Get SlimesExplosed
      (bind _asbp_judger (cast `/Game/LianJiaCheng/Blueprint/Judger/BP_Judger` (`self.Judger`)))
      (for _array_element (`/Game/LianJiaCheng/Blueprint/Judger/BP_Judger.AllSlimes` _asbp_judger)
        (`/Engine/EditorBlueprintResources/StandardMacros.IsValid` _array_element
          (:`Is Valid`
            (bind _asbp_slime_parent (cast `/Game/LianJiaCheng/Blueprint/Slime/BP_Slime_Parent` _array_element))
            (if (< (`self.GetDistanceTo` _asbp_slime_parent self) (`self.CreeperExplosionEffectRadius`))
              ;[1 1 1] Launch SlimesExplosed
              (`Character.LaunchCharacter` _asbp_slime_parent (* (`KismetMathLibrary.RandomUnitVectorInConeInDegrees` (0.0 0.0 1.0) 120.0) 2000.0) false false)
              ;[1 1 1] Add to Array
              (`KismetArrayLibrary.Array_Add` (`self.SlimesExplosed`) _asbp_slime_parent)
              (else
                ;[1 1 1] Launch SlimesUnExplosed
                (`Character.LaunchCharacter` _asbp_slime_parent (* (`KismetMathLibrary.GetUpVector` (struct)) 1000.0) false false)))))))
    (:`then_4`
      ;[1 1 1] SlimesExplosed Die
      ;;[1 1 1] SlimesExplosed Flying Time
      (`KismetSystemLibrary.Delay` 1.0)
      (for _array_element_2 (`self.SlimesExplosed`)
        (`/Engine/EditorBlueprintResources/StandardMacros.IsValid` _array_element_2
          (:`Is Valid`
            (bind _asbp_slime_parent_2 (cast `/Game/LianJiaCheng/Blueprint/Slime/BP_Slime_Parent` _array_element_2))
            (`/Game/LianJiaCheng/Blueprint/Slime/BP_Slime_Parent.Die` _asbp_slime_parent_2 "NewEnumerator0")
            ;[1 1 1] End CardEffect
            (`self.K2_DestroyActor`)))))))

(fn `UserConstructionScript`)