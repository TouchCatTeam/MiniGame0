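; Gameplay cue actor for the Nuwa's Hand card: for a limited duration, the player clicks in the world to create slimes.
; StartNuwa shows a target decal that tracks the mouse trace, and each click that hits queues a radius-scaled particle effect.
; Tick counts down parallel component/timer queues, spawning and launching a slime of random side and class before removing each effect.
; The actor destroys itself once time is up and both queues drain.
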(event `Start Nuwa`
  (params (DotTargetRadius :type "Float (double-precision)" :default 64.0) (NuwasHandEffectRadius :type "Float (double-precision)" :default 150.0))
  (set `self.NuwasHandEffectRadius` NuwasHandEffectRadius)
  (`|ExecutionSequence`
    (:`then_0`
      ;[1 1 1] init
      (set `self.IsNuwa` true))
    (:`then_1`
      ;[1 1 1] Spawn DotTaget
      (bind _returnvalue (`GameplayStatics.SpawnDecalAtLocation` "/Game/LianJiaCheng/Material/M_DotTarget.M_DotTarget" (`KismetMathLibrary.Conv_DoubleToVector` DotTargetRadius) (+ (`self.K2_GetActorLocation` self) (`KismetMathLibrary.MakeVector` 0.0 0.0 20.0))))
      (set `self.DotTargetDecal` _returnvalue))
    (:`then_2`
      ;[1 1 1] End1
      (`KismetSystemLibrary.Delay` (`self.Duration`))
      (set `self.IsNuwa` false)
      (set `self.IsEnd` true)
      (`ActorComponent.K2_DestroyComponent` (`self.DotTargetDecal`)))))

(event `self.ReceiveTick`
  (params (DeltaSeconds :type "Float (single-precision)"))
  (bind _psplayingdurationquene (`self.PSPlayingDurationQuene`))
  (bind _psdyingdurationquene (`self.PSDyingDurationQuene`))
  (bind _dottargetdecal (`self.DotTargetDecal`))
  (bind _output (`|GetArrayItem` (`self.PSPlayingQuene`)))
  (`|ExecutionSequence`
    (:`then_0`
      ;[1 1 1] Update Duration
      (for (_array_element _array_index) (`self.PSPlayingDurationQuene`)
        (`KismetArrayLibrary.Array_Set` (`self.PSPlayingDurationQuene`) _array_index (- _array_element DeltaSeconds))))
    (:`then_1`
      (for (_array_element_2 _array_index_2) (`self.PSDyingDurationQuene`)
        (`KismetArrayLibrary.Array_Set` (`self.PSDyingDurationQuene`) _array_index_2 (- _array_element_2 DeltaSeconds))))
    (:`then_2`
      ;[1 1 1] Update PS
      (if (> (`KismetArrayLibrary.Array_Length` _psplayingdurationquene) 0)
        (if (< (`|GetArrayItem` _psplayingdurationquene) 0.0)
          (`KismetArrayLibrary.Array_Remove` (`self.PSPlayingDurationQuene`))
          (`self.SpawnNewSlime` (`SceneComponent.K2_GetComponentLocation` _output))
          (`KismetArrayLibrary.Array_Add` (`self.PSDyingQuene`) _output)
          (`KismetArrayLibrary.Array_Add` (`self.PSDyingDurationQuene`) 0.5)
          (`KismetArrayLibrary.Array_Remove` (`self.PSPlayingQuene`)))))
    (:`then_3`
      (if (> (`KismetArrayLibrary.Array_Length` _psdyingdurationquene) 0)
        (if (< (`|GetArrayItem` _psdyingdurationquene) 0.0)
          (`KismetArrayLibrary.Array_Remove` (`self.PSDyingDurationQuene`))
          (`ActorComponent.K2_DestroyComponent` (`|GetArrayItem` (`self.PSDyingQuene`)))
          (`KismetArrayLibrary.Array_Remove` (`self.PSDyingQuene`)))))
    (:`then_4`
      ;[1 1 1] Update Mouse Hit Pos
      (bind _mousehitpos (`self.GetMouseHit`))
      (bind _output_get (set `self.CurrMousHitPos` _mousehitpos))
      ;[1 1 1] Update Decal Pos
      (`/Engine/EditorBlueprintResources/StandardMacros.IsValid` _dottargetdecal
        (:`Is Valid`
          (`SceneComponent.K2_SetWorldLocation` _dottargetdecal (+ _output_get (`KismetMathLibrary.MakeVector` 0.0 0.0 20.0)) false false))))
    (:`then_5`
      ;[1 1 1] Should End2?
      (if (`self.IsEnd`)
        (if (and (== (`KismetArrayLibrary.Array_Length` (`self.PSPlayingDurationQuene`)) 0) (== (`KismetArrayLibrary.Array_Length` (`self.PSDyingDurationQuene`)) 0))
          ;[1 1 1] End2
          (for _array_element_3 (`self.PSPlayingQuene`)
            (`ActorComponent.K2_DestroyComponent` _array_element_3))
          (for _array_element_4 (`self.PSDyingQuene`)
            (`ActorComponent.K2_DestroyComponent` _array_element_4))
          (`self.K2_DestroyActor`))))))

(event `InputAction|LMouseClick`
  (params (Key :type "Key Structure"))
  (:`Pressed`
    (if (`self.IsNuwa`)
      ;[1 1 1] Add in Quene
      (bind (_mousehitpos _ishit) (`self.GetMouseHit`))
      (if _ishit
        (bind _returnvalue (`GameplayStatics.SpawnEmitterAtLocation` "/Game/LianJiaCheng/Effect/MagicCircles2/ParticleSystems/PS_NuwasHand.PS_NuwasHand" (+ _mousehitpos (`KismetMathLibrary.MakeVector` 0.0 0.0 20.0)) (struct) (`KismetMathLibrary.Conv_DoubleToVector` (/ (`self.NuwasHandEffectRadius`) (`self.NuwasHandEffectOriginalRadius`)))))
        (`KismetArrayLibrary.Array_Add` (`self.PSPlayingQuene`) _returnvalue)
        (`KismetArrayLibrary.Array_Add` (`self.PSPlayingDurationQuene`) 2.0)))))

(fn `GetMouseHit`
  (returns (MouseHitPos :type "Vector Structure") (IsHit :type Boolean))
  (bind (_worldlocation _worlddirection) (`PlayerController.DeprojectMousePositionToWorld` (`GameplayStatics.GetPlayerController` 0)))
  (bind (_outhit _returnvalue) (`KismetSystemLibrary.LineTraceSingle` _worldlocation (+ _worldlocation (* _worlddirection 20000.0)) "TraceTypeQuery1"))
  (if _returnvalue
    (return (`.Location` (`GameplayStatics.BreakHitResult` _outhit)) true)
    (else
      (return (0.0 0.0 0.0) false))))

(fn `SpawnNewSlime`
  (params (SpawnPos :type "Vector Structure"))
  (bind _returnvalue (`|SpawnActorFromClass` "/Game/LianJiaCheng/Blueprint/Slime/BP_Slime_Parent.BP_Slime_Parent_C" (`KismetMathLibrary.Conv_VectorToTransform` SpawnPos) "Undefined" "OverrideRootScale" null null))
  (`/Engine/EditorBlueprintResources/StandardMacros.IsValid` _returnvalue
    (:`Is Valid`
      (switch `int` (`KismetMathLibrary.RandomIntegerInRange` 0 1)
        (:`0`
          (set `/Game/LianJiaCheng/Blueprint/Slime/BP_Slime_Parent.SideEnum` "NewEnumerator0" _returnvalue))
        (:`1`
          (set `/Game/LianJiaCheng/Blueprint/Slime/BP_Slime_Parent.SideEnum` "NewEnumerator1" _returnvalue)))
      (switch `int` (`KismetMathLibrary.RandomIntegerInRange` 0 3)
        (:`0`
          (set `/Game/LianJiaCheng/Blueprint/Slime/BP_Slime_Parent.ClassEnum` "NewEnumerator0" _returnvalue))
        (:`1`
          (set `/Game/LianJiaCheng/Blueprint/Slime/BP_Slime_Parent.ClassEnum` "NewEnumerator1" _returnvalue))
        (:`2`
          (set `/Game/LianJiaCheng/Blueprint/Slime/BP_Slime_Parent.ClassEnum` "NewEnumerator2" _returnvalue))
        (:`3`
          (set `/Game/LianJiaCheng/Blueprint/Slime/BP_Slime_Parent.ClassEnum` "NewEnumerator3" _returnvalue)))
      (`/Game/LianJiaCheng/Blueprint/Slime/BP_Slime_Parent.InitSlime` _returnvalue)
      (`Character.LaunchCharacter` _returnvalue (* (`KismetMathLibrary.RandomUnitVectorInConeInDegrees` (0.0 0.0 1.0) 60.0) 300.0) false false))))

(fn `UserConstructionScript`)