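; BP_GameplayCue_Parent is a base gameplay cue Blueprint that delivers one-shot audiovisual feedback when it begins play.
; BeginPlay runs three independent steps: a sound at the actor's location, an attached particle emitter, and a world camera shake centered on the actor.
; Each effect comes from a variable and plays only if that variable is valid, so any combination can be left unset.
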(event `self.ReceiveBeginPlay`
  (bind _soundtoplay (`self.SoundToPlay`))
  (bind _emittertemplatetoplay (`self.EmitterTemplateToPlay`))
  (bind _camerashaketoplay (`self.CameraShakeToPlay`))
  (`|ExecutionSequence`
    (:`then_0`
      ;[1 1 1] Play Sound
      (`/Engine/EditorBlueprintResources/StandardMacros.IsValid` _soundtoplay
        (:`Is Valid`
          (`GameplayStatics.SpawnSoundAtLocation` _soundtoplay (`self.K2_GetActorLocation` self) (struct) 1.0 1.0 0.0 null null))))
    (:`then_1`
      ;[1 1 1] Play Particle
      (`/Engine/EditorBlueprintResources/StandardMacros.IsValid` _emittertemplatetoplay
        (:`Is Valid`
          (`GameplayStatics.SpawnEmitterAttached` _emittertemplatetoplay null "None" (`self.K2_GetActorLocation` self)))))
    (:`then_2`
      ;[1 1 1] Play Camera Shake
      (if (`KismetSystemLibrary.IsValidClass` _camerashaketoplay)
        (`GameplayStatics.PlayWorldCameraShake` _camerashaketoplay (`self.K2_GetActorLocation` self))))))

(event `self.ReceiveDestroyed`)

(fn `UserConstructionScript`)