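; BP_Judgment decides breeding and combat deaths between slimes and searches for space for newborns.
; JudgeBirth (same side) and JudgeDeath (opposing sides) roll randomly against rate arrays indexed by both slime classes, with birth rates symmetric and death rates directional.
; TryGiveBirth walks expanding square rings around an actor, sphere-tracing each point for slimes.
; A free point goes to FindGiveBirthPos, which only breaks the search loops and spawns nothing.
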(event `/Game/LianJiaCheng/Blueprint/Judgment/BPI_Judgment.TryGiveBirth`
  (params (Obj :type "Actor Object Reference"))
  (bind _tmpfindpostotalcount (`self.TmpFindPosTotalCount`))
  (bind _tmpfindpostotalcount_2 (`self.TmpFindPosTotalCount`))
  (bind _tmpfindpostotalcount_3 (`self.TmpFindPosTotalCount`))
  ;[1 1 1] Init Layer
  (set `self.CurrPosLayer` 1)
  ;[1 1 1] Find Space For Each Layer
  (for _ (range (`self.CurrPosLayer`) (+ (`self.MaxPosLayer`) 1)) :!label _label
    (`|ExecutionSequence`
      (:`then_0`
        ;;[1 1 1] Init StartPos
        (set `self.StartPos` (+ (`self.K2_GetActorLocation` Obj) (`KismetMathLibrary.MakeVector` (* -1 (* (`self.CurrPosLayer`) (`self.LayerDis`))) (* (`self.CurrPosLayer`) (`self.LayerDis`)))))
        ;;[1 1 1] Init PosCount
        (set `self.TmpFindPosTotalCount` 1))
      (:`then_1`
        ;;[1 1 1] Layer++
        (set `self.CurrPosLayer` (+ (`self.CurrPosLayer`) 1)))
      (:`then_2`
        ;;[1 1 1] Find Space In This Layer
        (for _ (range (`self.TmpFindPosTotalCount`) (+ (* (`self.CurrPosLayer`) 8) 1)) :!label _label_2
          (`|ExecutionSequence`
            (:`then_0`
              (if (<= (`self.TmpFindPosTotalCount`) (* (`self.CurrPosLayer`) 2))
                (set `self.TmpDeltaVector` (`KismetMathLibrary.MakeVector` (`self.LayerDis`)))
                (bind _output_get (set `self.StartPos` (+ (`self.StartPos`) (`self.TmpDeltaVector`)) :!label _label_3))
                (bind _outhit (`KismetSystemLibrary.SphereTraceSingle` :`Start` (+ _output_get (0.0 0.0 20.0)) :`End` (+ _output_get (0.0 0.0 -20.0)) :`Radius` (`self.SphereTraceRadius`) :`TraceChannel` "TraceTypeQuery1" :`DrawDebugType` "ForDuration"))
                (cast `/Game/LianJiaCheng/Blueprint/Slime/BP_Slime_Parent` (`.HitActor` (`GameplayStatics.BreakHitResult` _outhit))
                  (:`CastFailed`
                    (`self.FindGiveBirthPos` _output_get)))
                (elif (and (> _tmpfindpostotalcount_2 (* (`self.CurrPosLayer`) 2)) (<= _tmpfindpostotalcount_2 (* (`self.CurrPosLayer`) 4)))
                  (set `self.TmpDeltaVector` (`KismetMathLibrary.MakeVector` 0.0 (* -1 (`self.LayerDis`))))
                  (goto _label_3)
                  (elif (and (> _tmpfindpostotalcount_3 (* (`self.CurrPosLayer`) 4)) (<= _tmpfindpostotalcount_3 (* (`self.CurrPosLayer`) 6)))
                    (set `self.TmpDeltaVector` (`KismetMathLibrary.MakeVector` (* -1 (`self.LayerDis`))))
                    (goto _label_3)
                    (elif (and (> _tmpfindpostotalcount (* (`self.CurrPosLayer`) 6)) (<= _tmpfindpostotalcount (* (`self.CurrPosLayer`) 8)))
                      (set `self.TmpDeltaVector` (`KismetMathLibrary.MakeVector` 0.0 (`self.LayerDis`)))
                      (goto _label_3))))))
            (:`then_1`
              ;;[1 1 1] PosCount++
              (set `self.TmpFindPosTotalCount` (+ (`self.TmpFindPosTotalCount`) 1)))))))))

(event `FindGiveBirthPos`
  (params (Pos :type "Vector Structure"))
  (`|ExecutionSequence`
    (:`then_0`
      (goto _label :!via `Break`))
    (:`then_1`
      (goto _label_2 :!via `Break`))))

(fn `JudgeBirth`
  (params (Obj1 :type "Actor Object Reference") (Obj2 :type "Actor Object Reference"))
  (returns (`Born?` :type Boolean))
  ;[1 1 1] Is Different Side?
  (bind _asbp_slime_parent (cast `/Game/LianJiaCheng/Blueprint/Slime/BP_Slime_Parent` Obj1))
  (bind _asbp_slime_parent_2 (cast `/Game/LianJiaCheng/Blueprint/Slime/BP_Slime_Parent` Obj2))
  (if (`|EnumEquality` (`/Game/LianJiaCheng/Blueprint/Slime/BP_Slime_Parent.SideEnum` _asbp_slime_parent) (`/Game/LianJiaCheng/Blueprint/Slime/BP_Slime_Parent.SideEnum` _asbp_slime_parent_2))
    ;[1 1 1] Switch Situations
    (switch `/Game/LianJiaCheng/Blueprint/Slime/E_Slime_ClassNum` (`/Game/LianJiaCheng/Blueprint/Slime/BP_Slime_Parent.ClassEnum` _asbp_slime_parent)
      (:`NewEnumerator0`
        (bind _classenum (`/Game/LianJiaCheng/Blueprint/Slime/BP_Slime_Parent.ClassEnum` _asbp_slime_parent_2))
        (switch `/Game/LianJiaCheng/Blueprint/Slime/E_Slime_ClassNum` _classenum
          (:`NewEnumerator0`
            (set `self.TmpBirthRate` (`|GetArrayItem` (`self.BirthHappenRateArray`))))
          (:`NewEnumerator1`
            (set `self.TmpBirthRate` (`|GetArrayItem` (`self.BirthHappenRateArray`) 1)))
          (:`NewEnumerator2`
            (set `self.TmpBirthRate` (`|GetArrayItem` (`self.BirthHappenRateArray`) 3)))
          (:`NewEnumerator3`
            (set `self.TmpBirthRate` (`|GetArrayItem` (`self.BirthHappenRateArray`) 6)))))
      (:`NewEnumerator1`
        (switch `/Game/LianJiaCheng/Blueprint/Slime/E_Slime_ClassNum` _classenum
          (:`NewEnumerator0`
            (set `self.TmpBirthRate` (`|GetArrayItem` (`self.BirthHappenRateArray`) 1)))
          (:`NewEnumerator1`
            (set `self.TmpBirthRate` (`|GetArrayItem` (`self.BirthHappenRateArray`) 2)))
          (:`NewEnumerator2`
            (set `self.TmpBirthRate` (`|GetArrayItem` (`self.BirthHappenRateArray`) 4)))
          (:`NewEnumerator3`
            (set `self.TmpBirthRate` (`|GetArrayItem` (`self.BirthHappenRateArray`) 7)))))
      (:`NewEnumerator2`
        (switch `/Game/LianJiaCheng/Blueprint/Slime/E_Slime_ClassNum` _classenum
          (:`NewEnumerator0`
            (set `self.TmpBirthRate` (`|GetArrayItem` (`self.BirthHappenRateArray`) 3)))
          (:`NewEnumerator1`
            (set `self.TmpBirthRate` (`|GetArrayItem` (`self.BirthHappenRateArray`) 4)))
          (:`NewEnumerator2`
            (set `self.TmpBirthRate` (`|GetArrayItem` (`self.BirthHappenRateArray`) 5)))
          (:`NewEnumerator3`
            (set `self.TmpBirthRate` (`|GetArrayItem` (`self.BirthHappenRateArray`) 8)))))
      (:`NewEnumerator3`
        (switch `/Game/LianJiaCheng/Blueprint/Slime/E_Slime_ClassNum` _classenum
          (:`NewEnumerator0`
            (set `self.TmpBirthRate` (`|GetArrayItem` (`self.BirthHappenRateArray`) 6)))
          (:`NewEnumerator1`
            (set `self.TmpBirthRate` (`|GetArrayItem` (`self.BirthHappenRateArray`) 7)))
          (:`NewEnumerator2`
            (set `self.TmpBirthRate` (`|GetArrayItem` (`self.BirthHappenRateArray`) 8)))
          (:`NewEnumerator3`
            (set `self.TmpBirthRate` (`|GetArrayItem` (`self.BirthHappenRateArray`) 9))))))
    (if (<= (`KismetMathLibrary.RandomFloatInRange` 0.0 100.0) (* (`self.TmpBirthRate`) 100.0))
      (return true)
      (else
        (return false)))))

(fn `JudgeDeath`
  (params (ObjAttacked :type "Actor Object Reference") (ObjAttacking :type "Actor Object Reference"))
  (returns (`Die?` :type Boolean))
  ;[1 1 1] Is Different Side?
  (bind _asbp_slime_parent (cast `/Game/LianJiaCheng/Blueprint/Slime/BP_Slime_Parent` ObjAttacked))
  (bind _asbp_slime_parent_2 (cast `/Game/LianJiaCheng/Blueprint/Slime/BP_Slime_Parent` ObjAttacking))
  (if (`|EnumInequality` (`/Game/LianJiaCheng/Blueprint/Slime/BP_Slime_Parent.SideEnum` _asbp_slime_parent) (`/Game/LianJiaCheng/Blueprint/Slime/BP_Slime_Parent.SideEnum` _asbp_slime_parent_2))
    ;[1 1 1] Switch Situations
    (switch `/Game/LianJiaCheng/Blueprint/Slime/E_Slime_ClassNum` (`/Game/LianJiaCheng/Blueprint/Slime/BP_Slime_Parent.ClassEnum` _asbp_slime_parent)
      (:`NewEnumerator0`
        (bind _classenum (`/Game/LianJiaCheng/Blueprint/Slime/BP_Slime_Parent.ClassEnum` _asbp_slime_parent_2))
        (switch `/Game/LianJiaCheng/Blueprint/Slime/E_Slime_ClassNum` _classenum
          (:`NewEnumerator0`
            (set `self.TmpDeathRate` (`|GetArrayItem` (`self.DeathRateArray`))))
          (:`NewEnumerator1`
            (set `self.TmpDeathRate` (`|GetArrayItem` (`self.DeathRateArray`) 1)))
          (:`NewEnumerator2`
            (set `self.TmpDeathRate` (`|GetArrayItem` (`self.DeathRateArray`) 2)))
          (:`NewEnumerator3`
            (set `self.TmpDeathRate` (`|GetArrayItem` (`self.DeathRateArray`) 3)))))
      (:`NewEnumerator1`
        (switch `/Game/LianJiaCheng/Blueprint/Slime/E_Slime_ClassNum` _classenum
          (:`NewEnumerator0`
            (set `self.TmpDeathRate` (`|GetArrayItem` (`self.DeathRateArray`) 4)))
          (:`NewEnumerator1`
            (set `self.TmpDeathRate` (`|GetArrayItem` (`self.DeathRateArray`) 5)))
          (:`NewEnumerator2`
            (set `self.TmpDeathRate` (`|GetArrayItem` (`self.DeathRateArray`) 6)))
          (:`NewEnumerator3`
            (set `self.TmpDeathRate` (`|GetArrayItem` (`self.DeathRateArray`) 7)))))
      (:`NewEnumerator2`
        (switch `/Game/LianJiaCheng/Blueprint/Slime/E_Slime_ClassNum` _classenum
          (:`NewEnumerator0`
            (set `self.TmpDeathRate` (`|GetArrayItem` (`self.DeathRateArray`) 8)))
          (:`NewEnumerator1`
            (set `self.TmpDeathRate` (`|GetArrayItem` (`self.DeathRateArray`) 9)))
          (:`NewEnumerator2`
            (set `self.TmpDeathRate` (`|GetArrayItem` (`self.DeathRateArray`) 10)))
          (:`NewEnumerator3`
            (set `self.TmpDeathRate` (`|GetArrayItem` (`self.DeathRateArray`) 11)))))
      (:`NewEnumerator3`
        (switch `/Game/LianJiaCheng/Blueprint/Slime/E_Slime_ClassNum` _classenum
          (:`NewEnumerator0`
            (set `self.TmpDeathRate` (`|GetArrayItem` (`self.DeathRateArray`) 12)))
          (:`NewEnumerator1`
            (set `self.TmpDeathRate` (`|GetArrayItem` (`self.DeathRateArray`) 13)))
          (:`NewEnumerator2`
            (set `self.TmpDeathRate` (`|GetArrayItem` (`self.DeathRateArray`) 14)))
          (:`NewEnumerator3`
            (set `self.TmpDeathRate` (`|GetArrayItem` (`self.DeathRateArray`) 15))))))
    (if (< (`KismetMathLibrary.RandomFloatInRange` 0.0 100.0) (* (`self.TmpDeathRate`) 100.0))
      (return true)
      (else
        (return false)))))

(fn `UserConstructionScript`)