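; Player pawn for a god-view card game: handles the zoom camera, energy and card input, and creates the HUD, swapping in a guide on level 1.
; Mouse-wheel zoom is clamped to a per-level sphere read from a data table.
; Left-click drives BP_CardRepertory's effect handler, spending energy when a placement indicator exists, or resolving a winding card otherwise; right-click cancels.
; Tick uses a Delay to regenerate energy at intervals.
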(event `Key|MouseScrollDown`
  (params (Key :type "Key Structure"))
  (:`Pressed`
    (bind _finaltargetpos (`self.ClampTargetPos` (+ (`SceneComponent.K2_GetComponentLocation` (`self.DefaultSceneRoot`)) (* (`SceneComponent.GetForwardVector` (`self.Camera`)) (* (`self.CameraZoomSpeed`) -1.0)))))
    (`SceneComponent.K2_SetWorldLocation` (`self.DefaultSceneRoot`) _finaltargetpos false false)))

(event `Key|MouseScrollUp`
  (params (Key :type "Key Structure"))
  (:`Pressed`
    (bind _finaltargetpos (`self.ClampTargetPos` (+ (`SceneComponent.K2_GetComponentLocation` (`self.DefaultSceneRoot`)) (* (`SceneComponent.GetForwardVector` (`self.Camera`)) (`self.CameraZoomSpeed`)))))
    (`SceneComponent.K2_SetWorldLocation` (`self.DefaultSceneRoot`) _finaltargetpos false false)))

(event `self.ReceiveBeginPlay`
  (`|ExecutionSequence`
    (:`then_0`
      ;[1 1 1] Add Player HUD
      (bind _returnvalue (`|CreateWidget` "/Game/XiaoHu/PlayHUD.PlayHUD_C" null self))
      (bind _output_get (set `self.IndexPlayHUD` _returnvalue))
      (`UserWidget.AddToViewport` _output_get 0))
    (:`then_1`
      ;[1 1 1] Get CardRepertory
      (bind _returnvalue_2 (`GameplayStatics.GetActorOfClass` "/Game/LianJiaCheng/Blueprint/Card/BP_CardRepertory.BP_CardRepertory_C"))
      (set `self.Index_CardRepertory` _returnvalue_2))
    (:`then_2`
      ;[1 1 1] Show Cursor
      (set `PlayerController.bShowMouseCursor` true (`GameplayStatics.GetPlayerController` 0)))
    (:`then_3`
      ;[1 1 1] Show Guide HUD
      (bind _returnvalue_3 (`GameplayStatics.GetCurrentLevelName` true))
      (if (== (- (`KismetStringLibrary.GetCharacterAsNumber` _returnvalue_3 5) 48) 1)
        (`Widget.SetVisibility` (`self.IndexPlayHUD`) "Hidden")
        (bind _returnvalue_4 (`|CreateWidget` "/Game/XiaoHu/UI_Guide.UI_Guide_C"))
        (`UserWidget.AddToViewport` _returnvalue_4 0)))
    (:`then_4`
      ;[1 1 1] Init Camera
      (`SceneComponent.K2_SetWorldRotation` (`self.Camera`) (`KismetMathLibrary.MakeRotator` 0.0 (`self.CameraInitPitch`)) false false))
    (:`then_5`
      ;[1 1 1] Refresh Camera Sphere
      (`self.RefreshCameraSphere`))))

(event `self.ReceiveTick`
  (params (DeltaSeconds :type "Float (single-precision)"))
  ;[1 1 1] 事件tick
  (`|ExecutionSequence`
    (:`then_0`
      (`KismetSystemLibrary.Delay` (`self.RecoverEnergyInterval`))
      (if (< (`self.Energy`) (`self.MaxEnergy`))
        (set `self.Energy` (+ (`self.Energy`) (`self.RecoverEnergyCount`)))))))

(event `Key|RightMouseButton` :consume false
  (params (Key :type "Key Structure"))
  (:`Pressed`
    (`/Game/XiaoHu/PlayHUD.取消释放` (`self.IndexPlayHUD`))))

(event `Key|LeftMouseButton` :consume false
  (params (Key :type "Key Structure"))
  (bind (_cardstyle _cardeffect _cardslimeside) (break `/Game/XiaoHu/Structure_Card` (`self.NowStructureCard`)))
  (bind (_cardstyle_2 _cardeffect_2 _cardslimeside_2) (break `/Game/XiaoHu/Structure_Card` (`self.NowStructureCard`)))
  (bind (_cardstyle_3 _cardeffect_3 _cardslimeside_3) (break `/Game/XiaoHu/Structure_Card` (`self.NowStructureCard`)))
  (bind (_cardstyle_4 _cardeffect_4 _cardslimeside_4) (break `/Game/XiaoHu/Structure_Card` (`self.NowStructureCard`)))
  (:`Pressed`
    (`/Engine/EditorBlueprintResources/StandardMacros.IsValid` (`/Game/LianJiaCheng/Blueprint/Card/BP_CardRepertory.TmpIndicator1` (`self.Index_CardRepertory`))
      (:`Is Valid`
        (set `self.Energy` (- (`self.Energy`) (`.Cost_13_8C4D60954A51523B0A7993B336AC467B` (break `/Game/XiaoHu/Structure_Card` (`self.NowStructureCard`)))))
        (`/Game/LianJiaCheng/Blueprint/Card/BP_CardRepertory.CardEffectHandler` (`self.Index_CardRepertory`) _cardeffect_4 "NewEnumerator1" _cardslimeside_4)
        (if (not (`|EnumEquality` _cardeffect_4 "NewEnumerator3"))
          (`/Game/LianJiaCheng/Blueprint/Card/BP_CardRepertory.CardEffectHandler` (`self.Index_CardRepertory`) _cardeffect "NewEnumerator7" _cardslimeside)
          (`/Game/XiaoHu/PlayHUD.所选卡使用后` (`self.IndexPlayHUD`))))
      (:`Is Not Valid`
        (if (`/Game/LianJiaCheng/Blueprint/Card/BP_CardRepertory.IsWinding` (`self.Index_CardRepertory`))
          (`/Game/LianJiaCheng/Blueprint/Card/BP_CardRepertory.CardEffectHandler` (`self.Index_CardRepertory`) _cardeffect_3 "NewEnumerator3" _cardslimeside_3)
          (`/Game/LianJiaCheng/Blueprint/Card/BP_CardRepertory.CardEffectHandler` (`self.Index_CardRepertory`) _cardeffect_2 "NewEnumerator2" _cardslimeside_2)
          (`/Game/XiaoHu/PlayHUD.所选卡使用后` (`self.IndexPlayHUD`)))))))

(fn `ClampTargetPos`
  (params (OriginalTargetPos :type "Vector Structure"))
  (returns (FinalTargetPos :type "Vector Structure"))
  (bind _cameraapproachablespherecenter (`self.CameraApproachableSphereCenter`))
  (if (> (`KismetMathLibrary.Abs` (`KismetMathLibrary.VSize` (- OriginalTargetPos (`self.CameraApproachableSphereCenter`)))) (`self.CameraApproachableSphereRadius`))
    (return (+ _cameraapproachablespherecenter (* (`KismetMathLibrary.Normal` (- OriginalTargetPos _cameraapproachablespherecenter)) (`self.CameraApproachableSphereRadius`))))
    (else
      (return OriginalTargetPos))))

(fn `GetMouseHit`
  (returns (HitActor :type "Actor Object Reference") (Location :type "Vector Structure"))
  (bind (_worldlocation _worlddirection) (`PlayerController.DeprojectMousePositionToWorld` (`GameplayStatics.GetPlayerController` 0)))
  (bind (_outhit _returnvalue) (`KismetSystemLibrary.LineTraceSingle` _worldlocation (+ _worldlocation (* _worlddirection 20000.0)) "TraceTypeQuery1"))
  (if _returnvalue
    (bind (_bblockinghit _binitialoverlap _time _distance _location _impactpoint _normal _impactnormal _physmat _hitactor) (`GameplayStatics.BreakHitResult` _outhit))
    (return _hitactor _location)))

(fn `RefreshCameraSphere`
  (bind _returnvalue (`GameplayStatics.GetCurrentLevelName` true))
  (bind _returnvalue_2 (`|GetDataTableRow` "/Game/XiaoHu/CSV_CameraApproachableSphere.CSV_CameraApproachableSphere" (`KismetStringLibrary.Conv_StringToName` _returnvalue))
    (:`then`
      (bind (_cameraapproachablespherecenter _cameraapproachablesphereradius) (break `/Game/XiaoHu/S_CameraApproachableSphere` _returnvalue_2))
      (set `self.CameraApproachableSphereCenter` _cameraapproachablespherecenter)
      (set `self.CameraApproachableSphereRadius` _cameraapproachablesphereradius))))

(fn `UserConstructionScript`)